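; Fuel pipe prop that gains a fire stream and a matching hidden hit box at each point where it is hit.
; Once the stream limit is reached, hits recycle existing streams and boxes in round-robin order.
; Each tick it syncs fuel flow to a valve wheel, toggling stream visibility.
; While fuel flows, it sends SetOnFireMessage to every actor overlapping the boxes.
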(event `self.ReceiveHit`
  (params (MyComp :type "PrimitiveComponent Object Reference") (Other :type "Actor Object Reference") (OtherComp :type "PrimitiveComponent Object Reference") (bSelfMoved :type Boolean) (HitLocation :type "Vector Structure") (HitNormal :type "Vector Structure") (NormalImpulse :type "Vector Structure") (Hit :type "HitResult Structure (by ref)"))
  ;[0 1 0] Adding Bullet Holes To The Pipes and Collision Boxes
  (if (== (`KismetArrayLibrary.Array_Length` (`self.FireStreams`)) (`self.MaxParticleStreams`))
    (`self.ReplaceOldStream` HitLocation HitNormal)
    (else
      (bind _index (`self.CreateParticleStream` HitLocation HitNormal))
      (`self.CreateParticleHitBox` _index))))

(event `self.ReceiveTick`
  (params (DeltaSeconds :type "Float (single-precision)"))
  (bind _activated (`/Game/Blueprints/Props/BP_ValveWheel.Activated` (`self.ValveWheel`)))
  ;[0 1 0] Whats Attempted Every Frame
  (`|ExecutionSequence`
    (:`then_0`
      ;;[0 0.03646 0] Use Valve Wheel To Control Fuel Flow
      (if (!= (`self.Fuel Flowing`) _activated)
        (`self.SetFuelFlow` _activated)))
    (:`then_1`
      ;;[0 0.03125 0] If the fire is flowing check for collisions and set things on fire
      (if (`self.Fuel Flowing`)
        (for _array_element (`self.FireHitBoxes`)
          (for _array_element_2 (`PrimitiveComponent.GetOverlappingActors` _array_element "/Script/Engine.Actor")
            (message `/Game/Blueprints/Interfaces/DamageableInterface.SetOnFire` _array_element_2)))))))

(fn `CreateParticleHitBox`
  (params (Index :type Integer))
  (bind _output (`|GetArrayItem` (`self.FireStreams`) Index))
  (bind _returnvalue (`AddComponent|NODE_AddBoxComponent-0`))
  (`BoxComponent.SetBoxExtent` _returnvalue (200.0 45.0 45.0) true)
  (`SceneComponent.K2_SetWorldLocationAndRotation` _returnvalue (`KismetSystemLibrary.GetComponentBounds` _output) (`KismetMathLibrary.Conv_VectorToRotator` (`SceneComponent.GetForwardVector` _output)) false false)
  (`PrimitiveComponent.SetCollisionResponseToChannel` _returnvalue "ECC_GameTraceChannel2" "ECR_Ignore")
  (`SceneComponent.SetHiddenInGame` _returnvalue true false)
  (`KismetArrayLibrary.Array_Add` (`self.FireHitBoxes`) _returnvalue))

(fn `CreateParticleStream`
  (params (`Hit Location` :type "Vector Structure") (`Hit Normal` :type "Vector Structure"))
  (returns (Index :type Integer))
  (bind _returnvalue (`GameplayStatics.SpawnEmitterAtLocation` (`self.ParticleStream`) `Hit Location` (`KismetMathLibrary.Conv_VectorToRotator` (* `Hit Normal` -1.0))))
  (if (not (`self.Fuel Flowing`))
    (`SceneComponent.SetVisibility` _returnvalue false false))
  (bind _returnvalue_2 (`KismetArrayLibrary.Array_Add` (`self.FireStreams`) _returnvalue))
  (return _returnvalue_2))

(fn `ReplaceOldStream`
  (params (`Hit Location` :type "Vector Structure") (`Hit Normal` :type "Vector Structure"))
  (bind _currentindex (`self.CurrentIndex`))
  (bind _output (`|GetArrayItem` (`self.FireStreams`) (`self.CurrentIndex`)))
  (`SceneComponent.K2_SetWorldLocationAndRotation` _output `Hit Location` (`KismetMathLibrary.Conv_VectorToRotator` (* `Hit Normal` -1.0)) false false)
  (`SceneComponent.K2_SetWorldLocationAndRotation` (`|GetArrayItem` (`self.FireHitBoxes`) (`self.CurrentIndex`)) (`KismetSystemLibrary.GetComponentBounds` _output) (`KismetMathLibrary.Conv_VectorToRotator` (`SceneComponent.GetForwardVector` _output)) false false)
  (set `self.CurrentIndex` (+ _currentindex 1))
  (if (== _currentindex (`self.MaxParticleStreams`))
    (set `self.CurrentIndex` 0)))

(fn `SetFuelFlow`
  (params (Value :type Boolean))
  (bind _output_get (set `self.Fuel Flowing` Value))
  (for _array_element (`self.FireStreams`)
    (`SceneComponent.SetVisibility` _array_element _output_get false)))

(fn `UserConstructionScript`)