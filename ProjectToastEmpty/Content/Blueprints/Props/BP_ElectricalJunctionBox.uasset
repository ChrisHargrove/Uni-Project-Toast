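; Junction box prop that breaks open once when a projectile overlaps it, electrocuting pawns in its shock zone at that moment.
; The construction script sizes and places the zone, and BeginPlay sets the lightning beam's target from the zone's X extent.
; StartShock swaps in the broken door, shows lightning and an effect, and sends an electrocute message to overlapping pawns.
; Tick hides only the lightning after the shock duration.
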(event `self.ReceiveActorBeginOverlap`
  (params (OtherActor :type "Actor Object Reference"))
  (if (not (`self.Triggered`))
    (cast `Projectile` OtherActor)
    (`self.StartShock`)))

(event `self.ReceiveBeginPlay`
  (bind _lightning (`self.Lightning`))
  (`ParticleSystemComponent.SetBeamTargetPoint` _lightning 0 (+ (* (* (`SceneComponent.GetForwardVector` _lightning) (.x (`BoxComponent.BoxExtent` (`self.ShockZone`)))) 2.0) (`SceneComponent.K2_GetComponentLocation` _lightning)) 0))

(event `self.ReceiveTick`
  (params (DeltaSeconds :type "Float (single-precision)"))
  (if (`self.Triggered`)
    (bind _output_get (set `self.ElapsedTime` (+ DeltaSeconds (`self.ElapsedTime`))))
    (if (>= _output_get (`self.Shock Duration`))
      (`SceneComponent.SetVisibility` (`self.Lightning`) false false))))

(fn `StartShock`
  (set `self.Triggered` true)
  (set `self.ElapsedTime` 0.0)
  (`SceneComponent.SetVisibility` (`self.Door`) false false)
  (`SceneComponent.SetVisibility` (`self.BrokenDoor`) true false)
  (`SceneComponent.SetVisibility` (`self.Lightning`) true false)
  (`SceneComponent.SetVisibility` (`self.Effect`) true false)
  (for _array_element (`PrimitiveComponent.GetOverlappingActors` (`self.ShockZone`) "/Script/Engine.Pawn")
    (message `/Game/Blueprints/Interfaces/DamageableInterface.Electrocute` _array_element)))

(fn `UserConstructionScript`
  (bind _shockzone (`self.ShockZone`))
  (`BoxComponent.SetBoxExtent` _shockzone (`self.ShockZoneSize`) true)
  (`SceneComponent.K2_SetWorldLocation` _shockzone (+ (`SceneComponent.K2_GetComponentLocation` (`self.BaseBox`)) (`self.ShockZonePosition`)) false false)
  (`SceneComponent.SetVisibility` (`self.BrokenDoor`) false false)
  (`SceneComponent.SetVisibility` (`self.Door`) true false))