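; BP_ValveWheel is an interactable valve wheel prop that turns back and forth as it is toggled.
; Each Interact flips Activated and plays or reverses the WheelRotation timeline, whose vector track feeds RotateWheel.
; RotateWheel sets the root component's relative roll from the track's X, reusing its world pitch and yaw.
; Highlight toggles custom depth rendering on the Wheel component.
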(event `/Game/Blueprints/Interfaces/InteractableInterface.Interact`
  (bind _activated (`self.Activated`))
  (set `self.Activated` (not _activated))
  (if _activated
    (bind (_direction _wheelrotation) (`Timeline|WheelRotation` :!label _label)
      (:`Update`
        (`self.RotateWheel` _wheelrotation)))
    (else
      (goto _label :!via `Reverse`))))

(event `/Game/Blueprints/Interfaces/InteractableInterface.Highlight`
  (params (ShouldHighlight :type Boolean))
  (`PrimitiveComponent.SetRenderCustomDepth` (`self.Wheel`) ShouldHighlight))

(fn `RotateWheel`
  (params (InVec :type "Vector Structure"))
  (`SceneComponent.K2_SetRelativeRotation` (`self.DefaultSceneRoot`) (`KismetMathLibrary.MakeRotator` (.x InVec) (.pitch (`SceneComponent.K2_GetComponentRotation` (`self.DefaultSceneRoot`))) (.yaw (`SceneComponent.K2_GetComponentRotation` (`self.DefaultSceneRoot`)))) false false))

(fn `UserConstructionScript`)