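; BP_Light_02 is a prop light Blueprint whose point light can be on, off or flickering.
; BeginPlay sets the light's visibility from IsLightOn, and Tick reapplies it whenever ShouldFlash is false.
; While ShouldFlash is true, Tick drives a DoOnce-gated loop that waits a random time between MinimumFlashTime and MaximumFlashTime, toggles the light, then resets the gate.
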(event `self.ReceiveBeginPlay`
  (`SceneComponent.SetVisibility` (`self.PointLight`) (`self.IsLightOn`) false :!label _label))

(event `self.ReceiveTick`
  (params (DeltaSeconds :type "Float (single-precision)"))
  (if (`self.ShouldFlash`)
    (`/Engine/EditorBlueprintResources/StandardMacros.DoOnce` false :!label _label_2
      (:`Completed`
        (`KismetSystemLibrary.RetriggerableDelay` (`KismetMathLibrary.RandomFloatInRange` (`self.MinimumFlashTime`) (`self.MaximumFlashTime`)))
        (`SceneComponent.ToggleVisibility` (`self.PointLight`) false)
        (goto _label_2 :!via `Reset`)))
    (else
      (goto _label))))

(fn `UserConstructionScript`)