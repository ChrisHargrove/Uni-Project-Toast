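; Interactable locker prop whose door swings open once when the player interacts with it.
; Highlight toggles custom depth on the Shell and Door meshes while highlighting is allowed.
; The first interaction permanently disables highlighting, turns off the door's collision and plays the OpenDoor timeline, which drives the door's relative rotation.
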(event `/Game/Blueprints/Interfaces/InteractableInterface.Interact`
  (`/Engine/EditorBlueprintResources/StandardMacros.DoOnce` false
    (:`Completed`
      (`|ExecutionSequence`
        (:`then_0`
          (`self.InterruptHighlight`))
        (:`then_1`
          (bind (_direction _door_rotation) (`Timeline|OpenDoor`)
            (:`Update`
              (`self.RotateDoor` _door_rotation))))))))

(event `/Game/Blueprints/Interfaces/InteractableInterface.Highlight`
  (params (ShouldHighlight :type Boolean))
  (`self.HighlightObject` ShouldHighlight))

(fn `HighlightObject`
  (params (bValue :type Boolean))
  (if (`self.CanHighlight`)
    (`|ExecutionSequence`
      (:`then_0`
        (`PrimitiveComponent.SetRenderCustomDepth` (`self.Shell`) bValue))
      (:`then_1`
        (`PrimitiveComponent.SetRenderCustomDepth` (`self.Door`) bValue)))))

(fn `InterruptHighlight`
  (bind _door (`self.Door`))
  (bind _output_get (set `self.CanHighlight` false))
  (`|ExecutionSequence`
    (:`then_0`
      (`PrimitiveComponent.SetRenderCustomDepth` (`self.Shell`) _output_get))
    (:`then_1`
      (`PrimitiveComponent.SetRenderCustomDepth` _door _output_get))
    (:`then_2`
      (`PrimitiveComponent.SetCollisionEnabled` _door "NoCollision"))))

(fn `RotateDoor`
  (params (InVec :type "Vector Structure"))
  (`SceneComponent.K2_SetRelativeRotation` (`self.Door`) (`KismetMathLibrary.MakeRotator` (.x InVec) (.y InVec) (.z InVec)) false false))

(fn `UserConstructionScript`)