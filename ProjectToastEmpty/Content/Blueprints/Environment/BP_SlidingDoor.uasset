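; Sliding double door that opens on trigger overlap when unlocked or when an optional keypad is activated.
; A DoorSlide timeline, with play rate set from SlideTime, moves the two panels in opposite directions.
; BeginPlay shows or hides the keypad according to HasKeypad.
; Overlap end reverses the timeline, and Tick also plays or reverses it every frame from the keypad state.
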(event `self.ReceiveBeginPlay`
  ;[0 0.99 0] On Play Start
  (`self.SetupDoor`))

(event `self.Trigger.OnComponentBeginOverlap`
  (params (OverlappedComponent :type "PrimitiveComponent Object Reference") (OtherActor :type "Actor Object Reference") (OtherComp :type "PrimitiveComponent Object Reference") (OtherBodyIndex :type Integer) (bFromSweep :type Boolean) (SweepResult :type "HitResult Structure (by ref)"))
  ;[0 1 0] Door Control
  ;;[1 1 1] On Player Overlap
  (if (not (`self.IsLocked`))
    (bind (_direction _door_slide) (`Timeline|DoorSlide` :!label _label)
      (:`Update`
        (`self.MoveDoor` _door_slide)))))

(event `self.Trigger.OnComponentEndOverlap`
  (params (OverlappedComponent :type "PrimitiveComponent Object Reference") (OtherActor :type "Actor Object Reference") (OtherComp :type "PrimitiveComponent Object Reference") (OtherBodyIndex :type Integer))
  ;[0 1 0] Door Control
  ;;[1 1 1] On Player Overlap
  (goto _label :!via `Reverse`))

(event `self.ReceiveTick`
  (params (DeltaSeconds :type "Float (single-precision)"))
  ;[0 1 0] Door Control
  ;;[1 1 1] If Keypad Activated
  (bind _activated (`self.IsKeyPadActivated`))
  (if _activated
    (goto _label)
    (else
      (goto _label :!via `Reverse`))))

(fn `IsKeyPadActivated`
  (returns (Activated :type Boolean))
  (if (`self.HasKeypad`)
    (return (`/Game/Blueprints/Props/BP_Keypad.Activated` (`self.KeyPad`)))))

(fn `MoveDoor`
  (params (NewLocation :type "Vector Structure"))
  (`|ExecutionSequence`
    (:`then_0`
      (`SceneComponent.K2_SetRelativeLocation` (`self.Door_Right`) NewLocation false false))
    (:`then_1`
      (`SceneComponent.K2_SetRelativeLocation` (`self.Door_Left`) (* NewLocation -1) false false))))

(fn `SetupDoor`
  (`|ExecutionSequence`
    (:`then_0`
      (`TimelineComponent.SetPlayRate` (`self.DoorSlide`) (/ 1.0 (`self.SlideTime`))))
    (:`then_1`
      (`SceneComponent.SetVisibility` (`Actor.RootComponent` (`self.KeyPad`)) (`self.HasKeypad`) false))))

(fn `UserConstructionScript`)