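; Interactable locker prop whose door swings open once when the player interacts with it.
; Interact runs a single time, turning off highlighting and door collision, then playing a timeline that yaws the door open.
; Highlight toggles custom depth on the shell and door for an outline effect until the locker is used.
; A StartOpen option poses the door open at construction.
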(event `/Game/Chris/Interfaces/InteractableInterface.Interact`
  (params (Interactee :type "/Game/Chris/Characters/Character/BP_FPSCharacter Object Reference"))
  (`/Engine/EditorBlueprintResources/StandardMacros.DoOnce` false
    (:`Completed`
      (`|ExecutionSequence`
        (:`then_0`
          (`self.InterruptHighlight`))
        (:`then_1`
          (bind (_direction _rotation) (`Timeline|OpenDoor`)
            (:`Update`
              (`self.RotateDoor` _rotation))))))))

(event `/Game/Chris/Interfaces/InteractableInterface.Highlight`
  (params (ShouldHighlight :type Boolean))
  (`self.HighlightObject` ShouldHighlight))

(fn `HighlightObject`
  (params (bValue :type Boolean))
  (if (`self.CanHighlight`)
    (`|ExecutionSequence`
      (:`then_0`
        (`PrimitiveComponent.SetRenderCustomDepth` (`self.Shell`) bValue))
      (:`then_1`
        (`PrimitiveComponent.SetRenderCustomDepth` (`self.Door`) bValue)))))

(fn `InterruptHighlight`
  (bind _door (`self.Door`))
  (bind _output_get (set `self.CanHighlight` false))
  (`|ExecutionSequence`
    (:`then_0`
      (`PrimitiveComponent.SetRenderCustomDepth` (`self.Shell`) _output_get))
    (:`then_1`
      (`PrimitiveComponent.SetRenderCustomDepth` _door _output_get))
    (:`then_2`
      (`PrimitiveComponent.SetCollisionEnabled` _door "NoCollision"))))

(fn `RotateDoor`
  (params (NewRotation :type "Float (double-precision)"))
  (`SceneComponent.K2_SetRelativeRotation` (`self.Door`) (`KismetMathLibrary.RotatorFromAxisAndAngle` (0.0 0.0 1.0) NewRotation) false false))

(fn `UserConstructionScript`
  (if (`self.StartOpen`)
    (`SceneComponent.K2_SetRelativeRotation` (`self.Door`) (`KismetMathLibrary.RotatorFromAxisAndAngle` (0.0 0.0 1.0) 90.0) false false)))