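; BP_AmmoPickup is an interactable ammo prop that grants the interacting player a per-type quantity of ammo, then destroys itself.
; Interact proceeds only when CheckIfPlayerAmmoFull returns true, which, despite its name, means the matching ammo entry is below max.
; The construction script sets the icon texture for Standard and Burst, and hides the icon and swaps the mesh for Explosion.
; Highlight toggles custom depth rendering on the mesh.
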(event `/Game/Chris/Interfaces/InteractableInterface.Interact`
  (params (Interactee :type "/Game/Chris/Characters/Character/BP_FPSCharacter Object Reference"))
  (bind _ammotype (`self.AmmoType`))
  (bind _canpickup (`self.CheckIfPlayerAmmoFull` Interactee))
  (if _canpickup
    (switch `/Game/Chris/Characters/Character/AmmoType` _ammotype
      (:`NewEnumerator0`
        (set `self.AmmoCount` 30))
      (:`NewEnumerator1`
        (set `self.AmmoCount` 30))
      (:`NewEnumerator2`
        (set `self.AmmoCount` 50))
      (:`NewEnumerator3`
        (set `self.AmmoCount` 5))
      (:`NewEnumerator4`
        (set `self.AmmoCount` 1)))
    (`/Game/Chris/Characters/Character/BP_FPSCharacter.AddAmmoOfType` Interactee _ammotype (`self.AmmoCount`))
    (`self.K2_DestroyActor`)))

(event `/Game/Chris/Interfaces/InteractableInterface.Highlight`
  (params (ShouldHighlight :type Boolean))
  (`PrimitiveComponent.SetRenderCustomDepth` (`self.AmmoMesh`) ShouldHighlight))

(fn `CheckIfPlayerAmmoFull`
  (params (Interactee :type "/Game/Chris/Characters/Character/BP_FPSCharacter Object Reference"))
  (returns (CanPickup :type Boolean))
  (for _array_element (`/Game/Chris/Characters/Character/BP_FPSCharacter.AmmoData` Interactee)
    (bind (_ammotype _ammocount _maxammo) (break `/Game/Chris/Characters/Character/PlayerAmmoStructure` _array_element))
    (if (`|EnumEquality` _ammotype (`self.AmmoType`))
      (if (== _ammocount _maxammo)
        (return false)
        (else
          (return true))))))

(fn `UserConstructionScript`
  (bind _material (`self.Material`))
  (bind _returnvalue (`DecalComponent.CreateDynamicMaterialInstance` (`self.AmmoIcon`)))
  (set `self.Material` _returnvalue)
  (switch `/Game/Chris/Characters/Character/AmmoType` (`self.AmmoType`)
    (:`NewEnumerator0`
      (`MaterialInstanceDynamic.SetTextureParameterValue` _material "Icon" "/Game/Chris/Textures/UI/SingleAmmoIcon.SingleAmmoIcon")
      (`SceneComponent.SetVisibility` (`self.AmmoIcon`) true false :!label _label))
    (:`NewEnumerator1`
      (`MaterialInstanceDynamic.SetTextureParameterValue` _material "Icon" "/Game/Chris/Textures/UI/TripleAmmoIcon.TripleAmmoIcon")
      (goto _label))
    (:`NewEnumerator4`
      (`SceneComponent.SetVisibility` (`self.AmmoIcon`) false false)
      (`StaticMeshComponent.SetStaticMesh` (`self.AmmoMesh`) (`|GetArrayItem` (`self.MeshChoices`) 1)))))