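; Tube light prop that switches to an alarm color around alarmed HooverBot AI sentries.
; The construction script creates a dynamic emissive material on the tube mesh and applies the configured color and intensity, matching the point light's color.
; Overlap events and a per-tick scan of overlapping bots check their alarm state.
; Both call SetColor, which recolors mesh material and point light together, to switch between alarm and normal colors.
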(event `self.ReceiveActorBeginOverlap`
  (params (OtherActor :type "Actor Object Reference"))
  (bind _asbp_ai_hoover_bot (cast `/Game/Chris/AI/BP_AI_HooverBot` OtherActor))
  (bind _output_get (set `self.RecentSentry` _asbp_ai_hoover_bot))
  (if (`/Game/Chris/AI/BP_AI_HooverBot.IsAlarmed` _output_get)
    (`self.SetColor` (`self.AlarmColor`))))

(event `self.ReceiveActorEndOverlap`
  (params (OtherActor :type "Actor Object Reference"))
  (cast `/Game/Chris/AI/BP_AI_HooverBot` OtherActor)
  (`self.SetColor` (`self.Color`)))

(event `self.ReceiveTick`
  (params (DeltaSeconds :type "Float (single-precision)"))
  (bind _arrayelement (`/Game/Chris/CustomMAcros.ForEachLoopWithBreakExit` (`self.GetOverlappingActors` "/Game/Chris/AI/BP_AI_HooverBot.BP_AI_HooverBot_C") :!label _label)
    (:`LoopBody`
      (bind _asbp_ai_hoover_bot (cast `/Game/Chris/AI/BP_AI_HooverBot` _arrayelement))
      (if (`/Game/Chris/AI/BP_AI_HooverBot.IsAlarmed` _asbp_ai_hoover_bot)
        (`self.SetColor` (`self.AlarmColor`))
        (goto _label :!via `Break`)))
    (:`Completed`
      (`self.SetColor` (`self.Color`)))))

(fn `SetColor`
  (params (`New Color` :type "Color Structure"))
  (bind _returnvalue (`KismetMathLibrary.Conv_ColorToLinearColor` `New Color`))
  (bind _asmaterial_instance_dynamic (cast `MaterialInstanceDynamic` (`PrimitiveComponent.GetMaterial` (`self.SM_TubeLight`) 0)))
  (`MaterialInstanceDynamic.SetVectorParameterValue` _asmaterial_instance_dynamic "LightColor" _returnvalue)
  (`LightComponent.SetLightColor` (`self.PointLight`) _returnvalue true))

(fn `UserConstructionScript`
  (bind _returnvalue (`PrimitiveComponent.CreateDynamicMaterialInstance` (`self.SM_TubeLight`) 0 "/Game/Chris/Materials/M_EmmisiveLight.M_EmmisiveLight" "None"))
  (`MaterialInstanceDynamic.SetVectorParameterValue` _returnvalue "LightColor" (`KismetMathLibrary.Conv_ColorToLinearColor` (`self.Color`)))
  (`MaterialInstanceDynamic.SetScalarParameterValue` _returnvalue "Intensity" (`self.Intensity`))
  (`LightComponent.SetLightColor` (`self.PointLight`) (`KismetMathLibrary.Conv_ColorToLinearColor` (`self.Color`)) true))