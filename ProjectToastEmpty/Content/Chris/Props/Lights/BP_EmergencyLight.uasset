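; Emergency light prop with a spinning reflector and two spotlights that can be switched on or off.
; Activate and Deactivate toggle both spotlights' visibility and set the IsActivated flag, which the construction script applies to preview the state in the editor.
; While activated, Tick yaws the reflector mesh at SpinSpeed, scaled by delta time.
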(event `self.ReceiveTick`
  (params (DeltaSeconds :type "Float (single-precision)"))
  (bind _sm_reflector (`self.SM_Reflector`))
  (if (`self.IsActivated`)
    (`SceneComponent.K2_SetRelativeRotation` _sm_reflector (`KismetMathLibrary.MakeRotator` (.roll (`SceneComponent.RelativeRotation` _sm_reflector)) (.pitch (`SceneComponent.RelativeRotation` _sm_reflector)) (+ (.yaw (`SceneComponent.RelativeRotation` _sm_reflector)) (* (`self.SpinSpeed`) DeltaSeconds))) false false)))

(fn `Activate`
  (`SceneComponent.SetVisibility` (`self.SpotLight1`) true false)
  (`SceneComponent.SetVisibility` (`self.SpotLight`) true false)
  (set `self.IsActivated` true))

(fn `Deactivate`
  (`SceneComponent.SetVisibility` (`self.SpotLight1`) false false)
  (`SceneComponent.SetVisibility` (`self.SpotLight`) false false)
  (set `self.IsActivated` false))

(fn `UserConstructionScript`
  (if (`self.IsActivated`)
    (`self.Activate`)
    (else
      (`self.Deactivate`))))