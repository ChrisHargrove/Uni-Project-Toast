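; A light prop Blueprint with two rect lights that can stay steadily on or off, or flicker at random.
; BeginPlay sets both lights' visibility from IsLightOn, and Tick reapplies it whenever ShouldFlash is false.
; While ShouldFlash is true, a DoOnce gates a random delay, then toggles both lights, plays an attached flicker sound and resets itself to repeat.
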(event `self.ReceiveBeginPlay`
  (bind _islighton (`self.IsLightOn`))
  (`SceneComponent.SetVisibility` (`self.RectLight`) _islighton false :!label _label)
  (`SceneComponent.SetVisibility` (`self.RectLight1`) _islighton false))

(event `self.ReceiveTick`
  (params (DeltaSeconds :type "Float (single-precision)"))
  (if (`self.Should Flash`)
    (`/Engine/EditorBlueprintResources/StandardMacros.DoOnce` false :!label _label_2
      (:`Completed`
        (`KismetSystemLibrary.RetriggerableDelay` (`KismetMathLibrary.RandomFloatInRange` (`self.Minimum Flash Time`) (`self.Maximum Flash Time`)))
        (`SceneComponent.ToggleVisibility` (`self.RectLight`) false)
        (`SceneComponent.ToggleVisibility` (`self.RectLight1`) false)
        (`GameplayStatics.SpawnSoundAttached` "/Game/Chris/Sounds/LightFlicker.LightFlicker" (`self.Root`) "None" (0.0 0.0 0.0) (struct) "SnapToTarget" false 1.0 1.0 0.0 "/Game/Chris/Sounds/AttenuationSettings/SoundAttentuation.SoundAttentuation" null)
        (goto _label_2 :!via `Reset`)))
    (else
      (goto _label))))

(fn `UserConstructionScript`)