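; BP_PowerCore is an interactable power core prop that the interacting actor can pick up.
; When not locked, Interact calls TogglePowerCore on the interactee, clears the highlight and destroys the prop.
; Highlighting toggles custom depth rendering on the casing, handle and core meshes, and is also ignored while locked.
; Helper functions set collision on all those parts and set the locked state.
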(event `/Game/Chris/Interfaces/InteractableInterface.Interact`
  (params (Interactee :type "/Game/Chris/Characters/Character/BP_FPSCharacter Object Reference"))
  (if (not (`self.IsLocked`))
    (`/Game/Chris/Characters/Character/BP_FPSCharacter.TogglePowerCore` Interactee true)
    (`self.HighlightObject` false)
    (`self.K2_DestroyActor`)))

(event `/Game/Chris/Interfaces/InteractableInterface.Highlight`
  (params (ShouldHighlight :type Boolean))
  (if (not (`self.IsLocked`))
    (`self.HighlightObject` ShouldHighlight)))

(fn `HighlightObject`
  (params (`Should Highlight` :type Boolean))
  (`|ExecutionSequence`
    (:`then_0`
      (`PrimitiveComponent.SetRenderCustomDepth` (`self.BottomCasing`) `Should Highlight`))
    (:`then_1`
      (`PrimitiveComponent.SetRenderCustomDepth` (`self.TopCasing`) `Should Highlight`))
    (:`then_2`
      (`PrimitiveComponent.SetRenderCustomDepth` (`self.EastHandle`) `Should Highlight`))
    (:`then_3`
      (`PrimitiveComponent.SetRenderCustomDepth` (`self.WestHandle`) `Should Highlight`))
    (:`then_4`
      (`PrimitiveComponent.SetRenderCustomDepth` (`self.NorthHandle`) `Should Highlight`))
    (:`then_5`
      (`PrimitiveComponent.SetRenderCustomDepth` (`self.SouthHandle`) `Should Highlight`))
    (:`then_6`
      (`PrimitiveComponent.SetRenderCustomDepth` (`self.Core`) `Should Highlight`))))

(fn `LockPowerCore`
  (params (IsLocked :type Boolean))
  (set `self.IsLocked` IsLocked))

(fn `ToggleCollisions`
  (params (CollisionType :type "ECollisionEnabled Enum" :default "NoCollision"))
  (`|ExecutionSequence`
    (:`then_0`
      (`PrimitiveComponent.SetCollisionEnabled` (`self.BottomCasing`) CollisionType))
    (:`then_1`
      (`PrimitiveComponent.SetCollisionEnabled` (`self.TopCasing`) CollisionType))
    (:`then_2`
      (`PrimitiveComponent.SetCollisionEnabled` (`self.EastHandle`) CollisionType))
    (:`then_3`
      (`PrimitiveComponent.SetCollisionEnabled` (`self.WestHandle`) CollisionType))
    (:`then_4`
      (`PrimitiveComponent.SetCollisionEnabled` (`self.NorthHandle`) CollisionType))
    (:`then_5`
      (`PrimitiveComponent.SetCollisionEnabled` (`self.SouthHandle`) CollisionType))
    (:`then_6`
      (`PrimitiveComponent.SetCollisionEnabled` (`self.Core`) CollisionType))))

(fn `UserConstructionScript`)