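; BP_GrenadeShell is a grenade projectile that explodes when it hits an AI character or when its fuse runs out.
; A hit on a BP_AI_Character detonates it at the hit location, while other hits are ignored.
; Tick accumulates elapsed time and detonates it at the mesh's location after ExplosionDelay.
; Both paths spawn BP_Explosion with the shell's damage and radius settings, then destroy the shell.
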(event `self.ReceiveHit`
  (params (MyComp :type "PrimitiveComponent Object Reference") (Other :type "Actor Object Reference") (OtherComp :type "PrimitiveComponent Object Reference") (bSelfMoved :type Boolean) (HitLocation :type "Vector Structure") (HitNormal :type "Vector Structure") (NormalImpulse :type "Vector Structure") (Hit :type "HitResult Structure (by ref)"))
  (cast `/Game/Chris/AI/BP_AI_Character` (`.HitActor` (`GameplayStatics.BreakHitResult` Hit)))
  (`|SpawnActorFromClass` "/Game/Chris/Props/Effects/BP_Explosion.BP_Explosion_C" (`KismetMathLibrary.Conv_VectorToTransform` HitLocation) "Undefined" "OverrideRootScale" null (`self.MaxDamage`) (`self.MinDamage`) (`self.ExplosionRadius`) 2 null)
  (`self.K2_DestroyActor`))

(event `self.ReceiveTick`
  (params (DeltaSeconds :type "Float (single-precision)"))
  (if (< (`self.ElapsedTime`) (`self.ExplosionDelay`))
    (set `self.ElapsedTime` (+ DeltaSeconds (`self.ElapsedTime`)))
    (else
      (`|SpawnActorFromClass` "/Game/Chris/Props/Effects/BP_Explosion.BP_Explosion_C" (`KismetMathLibrary.Conv_VectorToTransform` (`SceneComponent.K2_GetComponentLocation` (`self.StaticMesh`))) "Undefined" "OverrideRootScale" null (`self.MaxDamage`) (`self.MinDamage`) (`self.ExplosionRadius`) 2 null)
      (`self.K2_DestroyActor`))))

(fn `UserConstructionScript`)