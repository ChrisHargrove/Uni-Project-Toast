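; Fuel pipe prop that leaks damaging particle sprays where projectiles hit it.
; Hits spawn BP_ParticleSpray actors up to a cap, then reposition existing ones round-robin.
; Tick polls an optional valve wheel to toggle flow and accumulates burn time while leaking; on depletion it stops flow, destroys streams and locks the valve.
; The construction script tints the pipe through a dynamic material, and hits draw debug normal lines.
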(event `self.ReceiveBeginPlay`
  (bind _valvewheel (`self.ValveWheel`))
  (if (`KismetSystemLibrary.IsValid` _valvewheel)
    (if (!= (`self.Fuel Flowing`) (`/Game/Chris/Props/BP_ValveWheel.Activated` _valvewheel))
      (`/Game/Chris/Props/BP_ValveWheel.Interact` _valvewheel null))))

(event `self.ReceiveHit`
  (params (MyComp :type "PrimitiveComponent Object Reference") (Other :type "Actor Object Reference") (OtherComp :type "PrimitiveComponent Object Reference") (bSelfMoved :type Boolean) (HitLocation :type "Vector Structure") (HitNormal :type "Vector Structure") (NormalImpulse :type "Vector Structure") (Hit :type "HitResult Structure (by ref)"))
  ;[0 1 0] Adding Bullet Holes To The Pipes and Collision Boxes
  (cast `/Game/Chris/Props/Weapons/BP_Projectile` Other)
  (`KismetSystemLibrary.DrawDebugLine` HitLocation (+ HitLocation (* HitNormal 1000.0)) (struct :`R` 1.0 :`G` 0.13793 :`B` 0.763379 :`A` 1.0) 1000.0 3.0)
  (if (== (`KismetArrayLibrary.Array_Length` (`self.ParticleStreams`)) (`self.MaxParticleStreams`))
    (`self.ReplaceOldStream` HitLocation HitNormal)
    (else
      (`self.CreateParticleStream` HitLocation HitNormal))))

(event `self.ReceiveTick`
  (params (DeltaSeconds :type "Float (single-precision)"))
  (bind _activated (`/Game/Chris/Props/BP_ValveWheel.Activated` (`self.ValveWheel`)))
  ;[0 1 0] Whats Attempted Every Frame
  (`|ExecutionSequence`
    (:`then_0`
      ;;[0 0.03646 0] Use Valve Wheel To Control Fuel Flow
      (if (`KismetSystemLibrary.IsValid` (`self.ValveWheel`))
        (`|ExecutionSequence`
          (:`then_0`
            (if (!= (`self.Fuel Flowing`) _activated)
              (`self.SetFuelFlow` _activated))))))
    (:`then_1`
      ;;[0 0.03646 0] If Pipe hasnt run out of fuel then keep burning
      (if (and (`self.Fuel Flowing`) (> (`KismetArrayLibrary.Array_Length` (`self.ParticleStreams`)) 0))
        (bind _output_get (set `self.ElapsedBurnTime` (+ DeltaSeconds (`self.ElapsedBurnTime`))))
        (if (>= _output_get (`self.FuelBurnTime`))
          (bind _output_get_2 (set `self.HasFuel` false))
          (`self.SetFuelFlow` _output_get_2)
          (`self.ClearAllStreams`)
          (`/Game/Chris/Props/BP_ValveWheel.ResetValveWheel` (`self.ValveWheel`) _output_get_2 true))))))

(fn `ClearAllStreams`
  (for _array_element (`self.ParticleStreams`)
    (`self.K2_DestroyActor` _array_element)))

(fn `CreateParticleStream`
  (params (`Hit Location` :type "Vector Structure") (`Hit Normal` :type "Vector Structure"))
  (returns (Index :type Integer))
  (bind _returnvalue (`|SpawnActorFromClass` "/Game/Chris/Props/Effects/BP_ParticleSpray.BP_ParticleSpray_C" (`KismetMathLibrary.MakeTransform` `Hit Location` (`KismetMathLibrary.Conv_VectorToRotator` (* `Hit Normal` -1.0))) "Undefined" "OverrideRootScale" null (`self.ParticleTemplate`) (`self.ParticleType`) (`self.DamageAmount`) (`self.DamageDuration`) false null))
  (`/Game/Chris/Props/Effects/BP_ParticleSpray.SetActive` _returnvalue (`self.Fuel Flowing`))
  (bind _returnvalue_2 (`KismetArrayLibrary.Array_Add` (`self.ParticleStreams`) _returnvalue))
  (return _returnvalue_2))

(fn `ReplaceOldStream`
  (params (`Hit Location` :type "Vector Structure") (`Hit Normal` :type "Vector Structure"))
  (bind _currentindex (`self.CurrentIndex`))
  (`SceneComponent.K2_SetWorldLocationAndRotation` (`Actor.RootComponent` (`|GetArrayItem` (`self.ParticleStreams`) (`self.CurrentIndex`))) `Hit Location` (`KismetMathLibrary.Conv_VectorToRotator` (* `Hit Normal` -1.0)) false false)
  (set `self.CurrentIndex` (+ _currentindex 1))
  (if (== _currentindex (`self.MaxParticleStreams`))
    (set `self.CurrentIndex` 0)))

(fn `SetFuelFlow`
  (params (Value :type Boolean))
  (bind _output_get (set `self.Fuel Flowing` Value))
  (for _array_element (`self.ParticleStreams`)
    (`/Game/Chris/Props/Effects/BP_ParticleSpray.SetActive` _array_element _output_get)))

(fn `SetValveWheel`
  (params (ValveWheel :type "/Game/Chris/Props/BP_ValveWheel Object Reference"))
  (bind _output_get (set `self.ValveWheel` ValveWheel))
  (`/Game/Chris/Props/BP_ValveWheel.ResetValveWheel` _output_get (`self.Fuel Flowing`) false))

(fn `UserConstructionScript`
  (bind _returnvalue (`PrimitiveComponent.CreateDynamicMaterialInstance` (`self.SM_FuelPipe`) 0 "/Game/Chris/Materials/M_Lambert.M_Lambert" "None"))
  (`MaterialInstanceDynamic.SetVectorParameterValue` _returnvalue "BaseColor" (`KismetMathLibrary.Conv_ColorToLinearColor` (`self.PipeColor`))))