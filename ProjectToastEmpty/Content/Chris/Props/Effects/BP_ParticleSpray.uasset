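; BP_ParticleSpray is a fire or frost stream hazard that burns or freezes AI characters inside it.
; Construction applies the chosen particle template, and BeginPlay attaches the looping-stream sound matching ParticleType.
; Every Tick, it sends set-on-fire or freeze messages to BP_AI_Character actors overlapping StreamCollision.
; SetActive toggles particles, collision component and sound together, and the actor can optionally destroy itself when the particle system finishes.
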(event `DestroyParticleSpray`
  (params (PSystem :type "ParticleSystemComponent Object Reference"))
  (`self.K2_DestroyActor`))

(event `self.ReceiveBeginPlay`
  (bind _defaultsceneroot (`self.DefaultSceneRoot`))
  (if (`self.DestroyOnDeactivate`)
    (add `ParticleSystemComponent.OnSystemFinished` (`self.ParticleStream`) (delegate `DestroyParticleSpray`)))
  (switch `/Game/Chris/Props/Effects/EParticleSprayType` (`self.ParticleType`)
    (:`NewEnumerator0`
      (bind _returnvalue (`GameplayStatics.SpawnSoundAttached` "/Game/Chris/Sounds/high_pressure_flames.high_pressure_flames" _defaultsceneroot "None" (0.0 0.0 0.0) (struct) "SnapToTarget" false 1.0 1.0 0.0 "/Game/Chris/Sounds/AttenuationSettings/SoundAttentuation.SoundAttentuation" null false))
      (set `self.PipeSound` _returnvalue))
    (:`NewEnumerator1`
      (bind _returnvalue_2 (`GameplayStatics.SpawnSoundAttached` "/Game/Chris/Sounds/cryo_leak.cryo_leak" _defaultsceneroot "None" (0.0 0.0 0.0) (struct) "SnapToTarget" false 1.0 1.0 0.0 "/Game/Chris/Sounds/AttenuationSettings/SoundAttentuation.SoundAttentuation" null false))
      (set `self.PipeSound` _returnvalue_2))))

(event `self.ReceiveTick`
  (params (DeltaSeconds :type "Float (single-precision)"))
  (bind _duration (`self.Duration`))
  (for _array_element (`PrimitiveComponent.GetOverlappingActors` (`self.StreamCollision`) "/Game/Chris/AI/BP_AI_Character.BP_AI_Character_C")
    (switch `/Game/Chris/Props/Effects/EParticleSprayType` (`self.ParticleType`)
      (:`NewEnumerator0`
        (message `/Game/Chris/Interfaces/DamageableInterface.SetOnFire` _array_element (`self.Damage`) _duration))
      (:`NewEnumerator1`
        (message `/Game/Chris/Interfaces/DamageableInterface.Freeze` _array_element _duration)))))

(fn `SetActive`
  (params (IsActive :type Boolean))
  (bind _particlestream (`self.ParticleStream`))
  (bind _streamcollision (`self.StreamCollision`))
  (bind _pipesound (`self.PipeSound`))
  (if IsActive
    (`ActorComponent.Activate` _particlestream false)
    (`ActorComponent.Activate` _streamcollision false)
    (`AudioComponent.Play` _pipesound 0.0)
    (else
      (`ActorComponent.Deactivate` _particlestream)
      (`ActorComponent.Deactivate` _streamcollision)
      (`AudioComponent.Stop` _pipesound))))

(fn `UserConstructionScript`
  (`ParticleSystemComponent.SetTemplate` (`self.ParticleStream`) (`self.ParticleTemplate`)))