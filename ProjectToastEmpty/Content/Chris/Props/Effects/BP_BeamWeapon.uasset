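; Beam weapon actor that charges over time and fires a hitscan beam with damage scaled by charge.
; A looping timer counts charge up to five seconds, while the charge particle's finish swaps in full-charge visuals and sound.
; ActivateBeam line-traces forward to aim the beam, sends damage to the hit actor, and reports charge through an ammo-decrement dispatcher.
; The actor destroys itself when the beam effect finishes.
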(event `self.ReceiveBeginPlay`
  (bind _returnvalue (`KismetSystemLibrary.K2_SetTimerDelegate` (delegate `IncrementElapsedChargeTime`) 1.0 true))
  (set `self.ChargeTimer` _returnvalue)
  (add `ParticleSystemComponent.OnSystemFinished` (`self.BeamCharge`) (delegate `SwapChargeForFull`))
  (bind _returnvalue_2 (`GameplayStatics.SpawnSoundAttached` "/Game/Chris/Sounds/BeamEmitterChargeUp.BeamEmitterChargeUp" (`self.DefaultSceneRoot`) "None" (`SceneComponent.K2_GetComponentLocation` (`self.BeamFullCharge`)) (struct) "SnapToTarget" false 1.0 1.0 0.0 null null))
  (set `self.ChargingSound` _returnvalue_2)
  (add `ParticleSystemComponent.OnSystemFinished` (`self.Beam`) (delegate `DestroyBeamActor`)))

(event `DestroyBeamActor`
  (params (PSystem :type "ParticleSystemComponent Object Reference"))
  (`self.K2_DestroyActor`))

(event `SwapChargeForFull`
  (params (PSystem :type "ParticleSystemComponent Object Reference"))
  (bind _beamfullcharge (`self.BeamFullCharge`))
  (`SceneComponent.SetVisibility` _beamfullcharge true false)
  (bind _returnvalue (`GameplayStatics.SpawnSoundAttached` "/Game/Chris/Sounds/BeamEmitterFullCharge.BeamEmitterFullCharge" (`self.DefaultSceneRoot`) "None" (`SceneComponent.K2_GetComponentLocation` _beamfullcharge) (struct) "SnapToTarget" true 1.0 1.0 0.0 null null false))
  (set `self.FullyChargedSound` _returnvalue))

(event `IncrementElapsedChargeTime`
  (bind _result (`/Engine/EditorBlueprintResources/StandardMacros.IncrementInt` (`self.TotalChargeTime`))
    (:`  `
      (if (>= _result 5)
        (`KismetSystemLibrary.K2_ClearAndInvalidateTimerHandle` (`self.ChargeTimer`))))))

(fn `ActivateBeam`
  (params (InputPin :type "Delegate (by ref)"))
  (locals (LineTraceEnd :type "Vector Structure" :default (0.0 0.0 0.0)) (`World Location` :type "Vector Structure"))
  (bind _defaultsceneroot (`self.DefaultSceneRoot`))
  (bind _fullychargedsound (`self.FullyChargedSound`))
  (bind _chargingsound (`self.ChargingSound`))
  (bind _beam (`self.Beam`))
  (bind _returnvalue (`SceneComponent.K2_GetComponentLocation` _defaultsceneroot))
  (bind _returnvalue_2 (+ _returnvalue (* (`SceneComponent.GetForwardVector` _defaultsceneroot) (`self.MaximumDistance`))))
  (add `self.DecrementBeamAmmo` InputPin)
  (set `local.LineTraceEnd` _returnvalue_2)
  (bind (_outhit _returnvalue_3) (`KismetSystemLibrary.LineTraceSingle` :`Start` _returnvalue :`End` _returnvalue_2 :`TraceChannel` "TraceTypeQuery1" :`DrawDebugType` (`self.LineTraceDebug`) :`DrawTime` 5000.0))
  (`ActorComponent.SetActive` (`self.Beam`) true false)
  (if _returnvalue_3
    (bind (_bblockinghit _binitialoverlap _time _distance _location _impactpoint _normal _impactnormal _physmat _hitactor) (`GameplayStatics.BreakHitResult` _outhit))
    (`ParticleSystemComponent.SetBeamTargetPoint` _beam 0 _location 0)
    (else
      (`ParticleSystemComponent.SetBeamTargetPoint` _beam 0 (`local.LineTraceEnd`) 0)))
  (message `/Game/Chris/Interfaces/DamageableInterface.Damage` _hitactor (`KismetMathLibrary.MapRangeUnclamped` (`KismetMathLibrary.Conv_IntToDouble` (`self.TotalChargeTime`)) 0.0 5.0 0.0 (`self.Damage`)))
  (`self.DecrementBeamAmmo` (`self.TotalChargeTime`))
  (`|ExecutionSequence`
    (:`then_0`
      (if (`KismetSystemLibrary.IsValid` _fullychargedsound)
        (`AudioComponent.Stop` _fullychargedsound)))
    (:`then_1`
      (if (`KismetSystemLibrary.IsValid` _chargingsound)
        (`AudioComponent.Stop` _chargingsound)))
    (:`then_2`
      (`GameplayStatics.PlaySoundAtLocation` "/Game/Chris/Sounds/BeamEmitterFiring.BeamEmitterFiring" (`SceneComponent.K2_GetComponentLocation` (`self.BeamFullCharge`)) (struct) 1.0 1.0 0.0 "/Game/Chris/Sounds/AttenuationSettings/SoundAttentuation.SoundAttentuation" null null)
      (return))))

(fn `UserConstructionScript`)