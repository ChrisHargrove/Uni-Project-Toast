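; BP_Explosion is a self-destroying explosion actor with visual effects, sound, radial damage and physics force.
; On BeginPlay it plays an attenuated sound, sends RadialDamageMessage to overlapped actors whose origins lie within Radius, scaling damage linearly by distance, then fires a radial impulse.
; The construction script syncs the force radius and scales the particle system, whose finished event destroys the actor.
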(event `self.ReceiveBeginPlay`
  (bind _defaultsceneroot (`self.DefaultSceneRoot`))
  (add `ParticleSystemComponent.OnSystemFinished` (`self.ParticleSystem`) (delegate `Destroy Explosion Actor`))
  (`GameplayStatics.SpawnSoundAttached` "/Game/StarterContent/Audio/Explosion01.Explosion01" _defaultsceneroot "None" (0.0 0.0 0.0) (struct) "SnapToTarget" false 5.0 1.0 0.0 "/Game/Chris/Sounds/AttenuationSettings/ExplosionAttenuation.ExplosionAttenuation" null)
  (bind _outactors (`KismetSystemLibrary.SphereOverlapActors` (`SceneComponent.K2_GetComponentLocation` _defaultsceneroot) (`self.Radius`) (`self.OverlapActors`)))
  (for _array_element _outactors
    (bind _returnvalue (`self.GetDistanceTo` _array_element self))
    (if (not (> _returnvalue (`self.Radius`)))
      (message `/Game/Chris/Interfaces/DamageableInterface.RadialDamage` _array_element (`KismetMathLibrary.MapRangeUnclamped` _returnvalue 0.0 (`self.Radius`) (`self.MaxDamage`) (`self.MinDamage`)))))
  (`RadialForceComponent.FireImpulse` (`self.RadialForce`)))

(event `Destroy Explosion Actor`
  (params (PSystem :type "ParticleSystemComponent Object Reference"))
  (`self.K2_DestroyActor`))

(fn `UserConstructionScript`
  (bind _particlesystem (`self.ParticleSystem`))
  (set `RadialForceComponent.Radius` (`self.Radius`) (`self.RadialForce`))
  (`SceneComponent.SetRelativeScale3D` _particlesystem (* (`SceneComponent.RelativeScale3D` _particlesystem) (`self.ExplosionScale`))))