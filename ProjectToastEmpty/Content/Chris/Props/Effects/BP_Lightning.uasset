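; BP_Lightning is a lightning beam hazard that electrocutes AI characters inside a forward shock box.
; ShockZoneSize drives the box extent, beam end point and attenuation extents of the attached arc sound.
; Once Activate runs, Tick sends ElectrocuteMessage with damage, duration and instakill to every overlapping BP_AI_Character each frame.
; Duration also feeds the particle's LifeParam, and the actor stops its sound and destroys itself when the particle system finishes.
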(event `self.ReceiveBeginPlay`
  (add `ParticleSystemComponent.OnSystemFinished` (`self.Lightning`) (delegate `DestroyLightning`))
  (`self.SetDamageData` (`self.Damage`) (`self.Duration`) (`self.Instakill`))
  (`self.SetShockSize` (`self.Shock Zone Size`)))

(event `DestroyLightning`
  (params (PSystem :type "ParticleSystemComponent Object Reference"))
  (`AudioComponent.Stop` (`self.LightningSound`))
  (`self.K2_DestroyActor`))

(event `self.ReceiveTick`
  (params (DeltaSeconds :type "Float (single-precision)"))
  (if (`self.IsActive`)
    (for _array_element (`PrimitiveComponent.GetOverlappingActors` (`self.CollisionBox`) "/Game/Chris/AI/BP_AI_Character.BP_AI_Character_C")
      (if (`KismetSystemLibrary.IsValid` _array_element)
        (message `/Game/Chris/Interfaces/DamageableInterface.Electrocute` _array_element (`self.Damage`) (`self.Duration`) (`self.Instakill`))))))

(fn `Activate`
  (locals (SoundSettings :type "SoundAttenuationSettings Structure"))
  (bind _lightning (`self.Lightning`))
  (bind (_battenuate _bspatialize _battenuatewithlpf _benablelistenerfocus _benablefocusinterpolation _benableocclusion _busecomplexcollisionforocclusion _benablereverbsend _bapplynormalizationtostereosounds _benablelogfrequencyscaling _spatializationalgorithm _absorptionmethod _occlusiontracechannel _reverbsendmethod _omniradius _stereospread _lpfradiusmin _lpfradiusmax _customlowpassairabsorptioncurve _customhighpassairabsorptioncurve _lpffrequencyatmin _lpffrequencyatmax _hpffrequencyatmin _hpffrequencyatmax _focusazimuth _nonfocusazimuth _focusdistancescale _nonfocusdistancescale _focuspriorityscale _nonfocuspriorityscale _focusvolumeattenuation _nonfocusvolumeattenuation _focusattackinterpspeed _focusreleaseinterpspeed _occlusionlowpassfilterfrequency _occlusionvolumeattenuation _occlusioninterpolationtime _reverbwetlevelmin _reverbwetlevelmax _reverbdistancemin _reverbdistancemax _manualreverbsendlevel _customreverbsendcurve _pluginsettings _distancealgorithm _attenuationshape _dbattenuationatmax _attenuationshapeextents _coneoffset _falloffdistance _customattenuationcurve) (break `SoundAttenuationSettings` (`SoundAttenuation.Attenuation` (`self.LightningAttenuation`))))
  (`ActorComponent.SetActive` (`self.Lightning`) true false)
  (set `self.IsActive` true)
  (`ParticleSystemComponent.SetBeamTargetPoint` _lightning 0 (+ (`SceneComponent.K2_GetComponentLocation` _lightning) (* (`SceneComponent.GetForwardVector` _lightning) (* (.x (`self.Shock Zone Size`)) 2.0))) 0)
  (bind _output_get (set `local.SoundSettings` (make `SoundAttenuationSettings` _battenuate _bspatialize _battenuatewithlpf _benablelistenerfocus _benablefocusinterpolation _benableocclusion _busecomplexcollisionforocclusion _benablereverbsend _bapplynormalizationtostereosounds _benablelogfrequencyscaling _spatializationalgorithm _absorptionmethod _occlusiontracechannel _reverbsendmethod _omniradius _stereospread _lpfradiusmin _lpfradiusmax _customlowpassairabsorptioncurve _customhighpassairabsorptioncurve _lpffrequencyatmin _lpffrequencyatmax _hpffrequencyatmin _hpffrequencyatmax _focusazimuth _nonfocusazimuth _focusdistancescale _nonfocusdistancescale _focuspriorityscale _nonfocuspriorityscale _focusvolumeattenuation _nonfocusvolumeattenuation _focusattackinterpspeed _focusreleaseinterpspeed _occlusionlowpassfilterfrequency _occlusionvolumeattenuation _occlusioninterpolationtime _reverbwetlevelmin _reverbwetlevelmax _reverbdistancemin _reverbdistancemax _manualreverbsendlevel _customreverbsendcurve _pluginsettings _distancealgorithm _attenuationshape _dbattenuationatmax (`self.Shock Zone Size`) _coneoffset _falloffdistance _customattenuationcurve)))
  (bind _returnvalue (`GameplayStatics.SpawnSoundAttached` "/Game/Chris/Sounds/electric_arc.electric_arc" (`self.CollisionBox`) "None" (0.0 0.0 0.0) (struct) "SnapToTarget" false 1.0 1.0 0.0 "/Game/Chris/Sounds/AttenuationSettings/LightningAttenuation.LightningAttenuation" null))
  (bind _output_get_2 (set `self.LightningSound` _returnvalue))
  (`AudioComponent.AdjustAttenuation` _output_get_2 _output_get))

(fn `SetDamageData`
  (params (Damage :type "Float (double-precision)") (Duration :type "Float (double-precision)") (Instakill :type Boolean))
  (bind _output_get (set `self.Duration` Duration))
  (`ParticleSystemComponent.SetFloatParameter` (`self.Lightning`) "LifeParam" _output_get)
  (set `self.Damage` Damage)
  (set `self.Instakill` Instakill))

(fn `SetShockSize`
  (params (`New Size` :type "Vector Structure"))
  (bind _output_get (set `self.Shock Zone Size` `New Size`))
  (`BoxComponent.SetBoxExtent` (`self.CollisionBox`) _output_get true)
  (`SceneComponent.K2_SetRelativeLocation` (`self.CollisionBox`) (`KismetMathLibrary.MakeVector` (.x _output_get)) false false))

(fn `UserConstructionScript`
  (bind _lightning (`self.Lightning`))
  (bind _shock_zone_size (`self.Shock Zone Size`))
  (`BoxComponent.SetBoxExtent` (`self.CollisionBox`) _shock_zone_size true)
  (`SceneComponent.K2_SetRelativeLocation` (`self.CollisionBox`) (`KismetMathLibrary.MakeVector` (.x _shock_zone_size)) false false)
  (`ParticleSystemComponent.SetBeamTargetPoint` _lightning 0 (+ (`SceneComponent.K2_GetComponentLocation` _lightning) (* (`SceneComponent.GetForwardVector` _lightning) (* (.x (`self.Shock Zone Size`)) 2.0))) 0))