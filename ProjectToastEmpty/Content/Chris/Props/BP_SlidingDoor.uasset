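; Sliding double door that opens while the player overlaps its trigger and closes when they leave, unless locked.
; Tick polls the overlap and plays or reverses the DoorSlide timeline, which moves the two panels in opposite directions, with a sound.
; An optional linked keypad's Activated state is copied into IsLocked every frame.
; The construction script detects the keypad and derives the timeline play rate from SlideTime.
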(event `self.ReceiveTick`
  (params (DeltaSeconds :type "Float (single-precision)"))
  (bind _returnvalue (`SceneComponent.K2_GetComponentLocation` (`self.Frame`)))
  ;[0 1 0] Door Control
  (`|ExecutionSequence`
    (:`then_0`
      (if (not (`self.IsLocked`))
        (if (and (`PrimitiveComponent.IsOverlappingActor` (`self.Trigger`) (`GameplayStatics.GetPlayerCharacter` 0)) (not (or (`self.IsOpen`) (`self.InTransition`))))
          (set `self.InTransition` true)
          (`GameplayStatics.PlaySoundAtLocation` "/Game/Chris/Sounds/DoorOpen-Close.DoorOpen-Close" _returnvalue (struct) 1.0 1.0 0.0 "/Game/Chris/Sounds/AttenuationSettings/SoundAttentuation.SoundAttentuation" null null)
          (bind (_direction _door_slide) (`Timeline|DoorSlide` :!via `PlayFromStart` :!label _label)
            (:`Update`
              (`self.MoveDoor` _door_slide))
            (:`Finished`
              (set `self.IsOpen` (not (`self.IsOpen`)))
              (set `self.InTransition` false))))))
    (:`then_1`
      (if (not (`self.IsLocked`))
        (if (and (not (`PrimitiveComponent.IsOverlappingActor` (`self.Trigger`) (`GameplayStatics.GetPlayerCharacter` 0))) (and (`self.IsOpen`) (not (`self.InTransition`))))
          (set `self.InTransition` true)
          (`GameplayStatics.PlaySoundAtLocation` "/Game/Chris/Sounds/DoorOpen-Close.DoorOpen-Close" _returnvalue (struct) 1.0 1.0 0.0 "/Game/Chris/Sounds/AttenuationSettings/SoundAttentuation.SoundAttentuation" null null)
          (goto _label :!via `ReverseFromEnd`))))
    (:`then_2`
      (`self.IsKeyPadActivated`))))

(fn `IsKeyPadActivated`
  (if (`self.HasKeypad`)
    (set `self.IsLocked` (`/Game/Chris/Props/BP_Keypad.Activated` (`self.KeyPad`)))))

(fn `MoveDoor`
  (params (NewLocation :type "Vector Structure"))
  (`|ExecutionSequence`
    (:`then_0`
      (`SceneComponent.K2_SetRelativeLocation` (`self.Door_Right`) NewLocation false false))
    (:`then_1`
      (`SceneComponent.K2_SetRelativeLocation` (`self.Door_Left`) (* NewLocation -1) false false))))

(fn `UserConstructionScript`
  (`|ExecutionSequence`
    (:`then_0`
      (if (`KismetSystemLibrary.IsValid` (`self.KeyPad`))
        (set `self.HasKeypad` true)
        (else
          (set `self.HasKeypad` false))))
    (:`then_1`
      (`TimelineComponent.SetPlayRate` (`self.DoorSlide`) (/ 1.0 (`self.SlideTime`))))))