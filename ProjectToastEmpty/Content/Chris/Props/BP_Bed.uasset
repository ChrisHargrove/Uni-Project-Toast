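; BP_Bed is a bed prop that displays a bed number from 1 to 6.
; The construction script creates a dynamic instance of MI_BedNumber on element 0 of the BedNumber component and stores it in BedNumberMaterial.
; A switch on the bed number then sets that material's Diffuse parameter to the matching number texture.
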(fn `UserConstructionScript`
  (bind _returnvalue (`PrimitiveComponent.CreateDynamicMaterialInstance` (`self.Bed_Number`) 0 "/Game/Chris/Materials/Instances/MI_BedNumber.MI_BedNumber" "None"))
  (bind _output_get (set `self.bedNumberMaterial` _returnvalue))
  (switch `int` (`self.BedNumber`)
    (:`1`
      (`MaterialInstanceDynamic.SetTextureParameterValue` _output_get "Diffuse" "/Game/Chris/Textures/01.01"))
    (:`2`
      (`MaterialInstanceDynamic.SetTextureParameterValue` _output_get "Diffuse" "/Game/Chris/Textures/02.02"))
    (:`3`
      (`MaterialInstanceDynamic.SetTextureParameterValue` _output_get "Diffuse" "/Game/Chris/Textures/03.03"))
    (:`4`
      (`MaterialInstanceDynamic.SetTextureParameterValue` _output_get "Diffuse" "/Game/Chris/Textures/04.04"))
    (:`5`
      (`MaterialInstanceDynamic.SetTextureParameterValue` _output_get "Diffuse" "/Game/Chris/Textures/05.05"))
    (:`6`
      (`MaterialInstanceDynamic.SetTextureParameterValue` _output_get "Diffuse" "/Game/Chris/Textures/06.06"))))