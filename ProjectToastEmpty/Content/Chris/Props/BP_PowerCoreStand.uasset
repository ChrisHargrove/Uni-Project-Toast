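; Interactable power core stand that accepts a power core carried by the interacting actor.
; Construction creates dynamic materials for both stand meshes with glow off, then hides and locks a child-actor power core.
; Interacting while empty toggles off the carrier's core, reveals the built-in one and raises the stand glow, rather than moving an actor.
; Highlighting sets custom depth on both stand meshes only while the stand is empty.
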(event `/Game/Chris/Interfaces/InteractableInterface.Interact`
  (params (Interactee :type "/Game/Chris/Characters/Character/BP_FPSCharacter Object Reference"))
  (if (`self.HasCore`)
    _
    (elif (`/Game/Chris/Characters/Character/BP_FPSCharacter.HasPowerCore` Interactee)
      (`/Game/Chris/Characters/Character/BP_FPSCharacter.TogglePowerCore` Interactee false)
      (`self.PlacePowerCore`))))

(event `/Game/Chris/Interfaces/InteractableInterface.Highlight`
  (params (ShouldHighlight :type Boolean))
  (if (not (`self.HasCore`))
    (`PrimitiveComponent.SetRenderCustomDepth` (`self.Stand`) ShouldHighlight)
    (`PrimitiveComponent.SetRenderCustomDepth` (`self.TopStand`) ShouldHighlight)))

(fn `PlacePowerCore`
  (set `self.HasCore` true)
  (`MaterialInstanceDynamic.SetScalarParameterValue` (`self.TopStandMaterial`) "GlowIntensity" 30.0)
  (`MaterialInstanceDynamic.SetScalarParameterValue` (`self.BottomStandMaterial`) "GlowIntensity" 30.0)
  (`SceneComponent.SetVisibility` (`self.PowerCore`) true false))

(fn `UserConstructionScript`
  (bind _powercore (`self.PowerCore`))
  (`|ExecutionSequence`
    (:`then_0`
      (bind _returnvalue (`PrimitiveComponent.CreateDynamicMaterialInstance` (`self.Stand`) 0 "/Game/Chris/Materials/Instances/Props/MI_PowerCoreStand.MI_PowerCoreStand" "None"))
      (set `self.BottomStandMaterial` _returnvalue)
      (bind _returnvalue_2 (`PrimitiveComponent.CreateDynamicMaterialInstance` (`self.TopStand`) 0 "/Game/Chris/Materials/Instances/Props/MI_PowerCoreStand.MI_PowerCoreStand" "None"))
      (set `self.TopStandMaterial` _returnvalue_2))
    (:`then_1`
      (`MaterialInstanceDynamic.SetScalarParameterValue` (`self.TopStandMaterial`) "GlowIntensity" 0.0)
      (`MaterialInstanceDynamic.SetScalarParameterValue` (`self.BottomStandMaterial`) "GlowIntensity" 0.0))
    (:`then_2`
      (`SceneComponent.ToggleVisibility` _powercore false)
      (bind _asbp_power_core (cast `/Game/Chris/Props/BP_PowerCore` (`ChildActorComponent.ChildActor` _powercore)))
      (`/Game/Chris/Props/BP_PowerCore.LockPowerCore` _asbp_power_core true))))