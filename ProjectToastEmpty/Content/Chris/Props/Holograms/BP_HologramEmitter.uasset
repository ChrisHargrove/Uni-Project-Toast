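; A hologram emitter prop that displays a slowly or quickly spinning hologram of either a static or skeletal mesh.
; The construction script uses ShowSkeletalMesh to show one mesh component and hide the other, then applies the chosen mesh, scale and height offset.
; Each tick, RotateObject adds RotationSpeed times delta time to the visible component's world yaw.
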(event `self.ReceiveTick`
  (params (DeltaSeconds :type "Float (single-precision)"))
  (if (`self.ShowSkeletalMesh`)
    (`self.Rotate Object` (`self.HologramSkeletonObject`) DeltaSeconds)
    (else
      (`self.Rotate Object` (`self.HologramObject`) DeltaSeconds))))

(fn `Rotate Object`
  (params (`Target Object` :type "SceneComponent Object Reference") (`Delta Time` :type "Float (double-precision)"))
  (`SceneComponent.K2_SetWorldRotation` `Target Object` (`KismetMathLibrary.MakeRotator` (.roll (`SceneComponent.K2_GetComponentRotation` `Target Object`)) (.pitch (`SceneComponent.K2_GetComponentRotation` `Target Object`)) (+ (.yaw (`SceneComponent.K2_GetComponentRotation` `Target Object`)) (* (`self.RotationSpeed`) `Delta Time`))) false false))

(fn `UserConstructionScript`
  (bind _hologramobject (`self.HologramObject`))
  (bind _hologramobject_2 (`self.HologramObject`))
  (bind _scale (`self.Scale`))
  (bind _hologramskeletonobject (`self.HologramSkeletonObject`))
  (bind _hologramskeletonobject_2 (`self.HologramSkeletonObject`))
  (if (`self.ShowSkeletalMesh`)
    (`SceneComponent.SetVisibility` _hologramskeletonobject true false)
    (`SceneComponent.SetVisibility` _hologramobject false false)
    (`SkinnedMeshComponent.SetSkinnedAssetAndUpdate` _hologramskeletonobject_2 (`self.HologramSkeleton`) true)
    (`SceneComponent.SetRelativeScale3D` _hologramskeletonobject_2 _scale)
    (`SceneComponent.K2_SetWorldLocation` _hologramskeletonobject_2 (`KismetMathLibrary.MakeVector` (.x (`SceneComponent.K2_GetComponentLocation` _hologramskeletonobject_2)) (.y (`SceneComponent.K2_GetComponentLocation` _hologramskeletonobject_2)) (+ (.z (`SceneComponent.K2_GetComponentLocation` _hologramskeletonobject_2)) (`self.HeightOffset`))) false false)
    (else
      (`SceneComponent.SetVisibility` _hologramskeletonobject false false)
      (`SceneComponent.SetVisibility` _hologramobject true false)
      (`StaticMeshComponent.SetStaticMesh` _hologramobject (`self.HologramMesh`))
      (`SceneComponent.SetRelativeScale3D` _hologramobject_2 _scale)
      (`SceneComponent.K2_SetWorldLocation` _hologramobject_2 (`KismetMathLibrary.MakeVector` (.x (`SceneComponent.K2_GetComponentLocation` _hologramobject_2)) (.y (`SceneComponent.K2_GetComponentLocation` _hologramobject_2)) (+ (.z (`SceneComponent.K2_GetComponentLocation` _hologramobject_2)) (`self.HeightOffset`))) false false))))