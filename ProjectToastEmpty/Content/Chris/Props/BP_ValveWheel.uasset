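; BP_ValveWheel is an interactable valve wheel prop that toggles between activated and deactivated when not locked.
; Interact flips the state, plays a sound and runs the WheelRotation timeline forward or backward, with RotateWheel turning the pivot around its local X axis.
; ResetValveWheel sets the activated and lock states, animating only when activated.
; Highlight toggles custom depth rendering on the wheel mesh.
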(event `ResetValveWheel`
  (params (Activated :type Boolean) (Lock :type Boolean))
  (set `self.IsLocked` Lock)
  (bind _output_get (set `self.Activated` Activated))
  (if _output_get
    (`GameplayStatics.PlaySoundAtLocation` "/Game/Chris/Sounds/ValveWheel.ValveWheel" (`SceneComponent.K2_GetComponentLocation` (`self.Root`)) (struct) 1.0 1.0 0.0 "/Game/Chris/Sounds/AttenuationSettings/SoundAttentuation.SoundAttentuation" null null :!label _label)
    (bind (_direction _rotation) (`Timeline|WheelRotation` :!label _label_2)
      (:`Update`
        (`self.RotateWheel` _rotation)))))

(event `/Game/Chris/Interfaces/InteractableInterface.Interact`
  (params (Interactee :type "/Game/Chris/Characters/Character/BP_FPSCharacter Object Reference"))
  (bind _activated (`self.Activated`))
  (if (not (`self.IsLocked`))
    (set `self.Activated` (not _activated))
    (if _activated
      (goto _label)
      (else
        (`GameplayStatics.PlaySoundAtLocation` "/Game/Chris/Sounds/ValveWheel.ValveWheel" (`SceneComponent.K2_GetComponentLocation` (`self.Root`)) (struct) 1.0 1.0 0.0 "/Game/Chris/Sounds/AttenuationSettings/SoundAttentuation.SoundAttentuation" null null)
        (goto _label_2 :!via `Reverse`)))))

(event `/Game/Chris/Interfaces/InteractableInterface.Highlight`
  (params (ShouldHighlight :type Boolean))
  (`PrimitiveComponent.SetRenderCustomDepth` (`self.Wheel`) ShouldHighlight))

(fn `RotateWheel`
  (params (Rotation :type "Float (double-precision)"))
  (`SceneComponent.K2_SetRelativeRotation` (`self.WheelRotationPoint`) (`KismetMathLibrary.RotatorFromAxisAndAngle` (1.0 0.0 0.0) Rotation) false false))

(fn `UserConstructionScript`)