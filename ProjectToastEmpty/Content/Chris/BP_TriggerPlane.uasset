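; BP_TriggerPlane is a directional trigger that spawns AI when the player character passes through it.
; On overlap, a dot product of the actor's and plane's forward vectors filters out actors not facing roughly the same way.
; For a BP_FPSCharacter, it calls SpawnAI on a random SpawnPoints entry, passing the plane's location or a zero vector, per SetPlayerLocation.
; The random index range includes the array length, so it can fall out of bounds.
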(event `self.Trigger.OnComponentBeginOverlap`
  (params (OverlappedComponent :type "PrimitiveComponent Object Reference") (OtherActor :type "Actor Object Reference") (OtherComp :type "PrimitiveComponent Object Reference") (OtherBodyIndex :type Integer) (bFromSweep :type Boolean) (SweepResult :type "HitResult Structure (by ref)"))
  (if (> (`KismetMathLibrary.Dot_VectorVector` (`self.GetActorForwardVector` OtherActor) (`SceneComponent.GetForwardVector` (`self.Root`))) 0.5)
    (`self.SpawnAI` OtherActor)))

(fn `SpawnAI`
  (params (Actor :type "Actor Object Reference"))
  (bind _returnvalue (`KismetArrayLibrary.Array_Length` (`self.SpawnPoints`)))
  (bind _output (`|GetArrayItem` (`self.SpawnPoints`) (`KismetMathLibrary.RandomIntegerInRange` 0 _returnvalue)))
  (if (> _returnvalue 0)
    (cast `/Game/Chris/Characters/Character/BP_FPSCharacter` Actor)
    (if (`self.SetPlayerLocation`)
      (`/Game/Chris/AI/BP_AI_SpawnPoint.SpawnAI` _output (`SceneComponent.K2_GetComponentLocation` (`self.Root`)))
      (else
        (`/Game/Chris/AI/BP_AI_SpawnPoint.SpawnAI` _output (0.0 0.0 0.0))))))

(fn `UserConstructionScript`)