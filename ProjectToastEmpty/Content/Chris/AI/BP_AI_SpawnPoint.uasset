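; AI spawn point actor that spawns a random pawn from its AICharacters list when its location is off the player's screen.
; SpawnAI runs only at zero cooldown, starting a looping timer before the screen check, and can pass an enemy search location to the spawned BP_AI_Character.
; IsOnScreen compares the projected location to viewport bounds.
; IncrementCooldown advances the cooldown, clearing the timer and resetting at TimeBetweenSpawns.
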(fn `IncrementCooldown`
  (bind _output_get (set `self.Cooldown` (+ (`self.Cooldown`) 0.5)))
  (if (>= _output_get (`self.TimeBetweenSpawns`))
    (`KismetSystemLibrary.K2_ClearAndInvalidateTimerHandle` (`self.CooldownTimer`))
    (set `self.Cooldown` 0.0)))

(fn `IsOnScreen`
  (returns (OnScreen :type Boolean))
  (bind (_x _y) (`KismetMathLibrary.BreakVector2D` (`WidgetLayoutLibrary.GetViewportSize`)))
  (bind (_x_2 _y_2) (`KismetMathLibrary.BreakVector2D` (`PlayerController.ProjectWorldLocationToScreen` (`GameplayStatics.GetPlayerController` 0) (`SceneComponent.K2_GetComponentLocation` (`self.DefaultSceneRoot`)) false)))
  (return (and (> _x_2 0.0) (> _y_2 0.0) (< _x_2 _x) (< _y_2 _y))))

(fn `SpawnAI`
  (params (`Enemy Location` :type "Vector Structure"))
  (returns (HasSpawned :type Boolean))
  (bind _ai_characters (`self.AI Characters`))
  (`|ExecutionSequence`
    (:`then_0`
      (if (== (`self.Cooldown`) 0.0)
        (goto _label :!via `Open`)
        (else
          (goto _label :!via `Close`))))
    (:`then_1`
      (`/Engine/EditorBlueprintResources/StandardMacros.Gate` true :!label _label
        (:`Exit`
          (bind _returnvalue (`KismetSystemLibrary.K2_SetTimerDelegate` (`|CreateDelegate` :!event `IncrementCooldown`) 0.5 true))
          (set `self.CooldownTimer` _returnvalue)
          (bind _onscreen (`self.IsOnScreen`))
          (if _onscreen
            (return false)
            (else
              (bind _returnvalue_2 (`AIBlueprintHelperLibrary.SpawnAIFromClass` (`|GetArrayItem` _ai_characters (`KismetMathLibrary.RandomIntegerInRange` 0 (- (`KismetArrayLibrary.Array_Length` _ai_characters) 1))) null (`SceneComponent.K2_GetComponentLocation` (`self.DefaultSceneRoot`))))
              (if (!= `Enemy Location` (0.0 0.0 0.0))
                (bind _asbp_ai_character (cast `/Game/Chris/AI/BP_AI_Character` _returnvalue_2))
                (`/Game/Chris/AI/BP_AI_Character.SetEnemySearchLocation` _asbp_ai_character `Enemy Location`)
                (return true)
                (else
                  (return true))))))))))

(fn `UserConstructionScript`
  (`parent.UserConstructionScript`))