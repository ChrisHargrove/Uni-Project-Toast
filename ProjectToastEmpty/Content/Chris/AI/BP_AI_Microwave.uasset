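; BP_AI_Microwave is a microwave AI character that explodes when its health runs out.
; Each tick it checks Health and advances a damage-over-time timer through IncrementDOTTimer.
; On death it unpossesses its AI controller and disables capsule collision.
; It then destroys its particle systems, spawns BP_Explosion at the capsule location using its explosion damage and radius, and destroys itself.
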(event `self.ReceiveTick`
  (params (DeltaSeconds :type "Float (single-precision)"))
  (bind _explosiondamage (`self.ExplosionDamage`))
  (`|ExecutionSequence`
    (:`then_0`
      (bind _isdead (`self.CheckForDeath`))
      (if _isdead
        (`/Engine/EditorBlueprintResources/StandardMacros.DoOnce` false
          (:`Completed`
            (`|ExecutionSequence`
              (:`then_0`
                (for _array_element (`self.ParticleSystems`)
                  (`ActorComponent.K2_DestroyComponent` _array_element)))
              (:`then_1`
                (`|SpawnActorFromClass` "/Game/Chris/Props/Effects/BP_Explosion.BP_Explosion_C" (`KismetMathLibrary.Conv_VectorToTransform` (`SceneComponent.K2_GetComponentLocation` (`self.CapsuleComponent`))) "Undefined" "OverrideRootScale" null _explosiondamage _explosiondamage (`self.ExplosionRadius`) 3 null)
                (`self.K2_DestroyActor`)))))))
    (:`then_1`
      (`self.IncrementDOTTimer` DeltaSeconds))))

(fn `CheckForDeath`
  (returns (IsDead :type Boolean))
  (if (<= (`self.Health`) 0.0)
    (if (not (`self.Unpossessed`))
      (`Controller.UnPossess` (`AIBlueprintHelperLibrary.GetAIController` self))
      (set `self.Unpossessed` true)
      (`PrimitiveComponent.SetCollisionEnabled` (`self.CapsuleComponent`) "NoCollision")
      (return true))
    (else
      (return false))))

(fn `UserConstructionScript`
  (`parent.UserConstructionScript`))