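; AI enemy character that takes damage, burns, electrocution and freezing, then dies and cleans itself up.
; Burn and shock attach bone particles and share a looping damage-over-time timer.
; Shock and freeze pause AI through blackboard, movement and animation; freeze also swaps in ice materials temporarily.
; Tick destroys the controller at zero health, then, when flagged NeedsRemoval, ragdolls and destroys the actor after it stays off screen for the decay time.
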(event `/Game/Chris/Interfaces/DamageableInterface.RadialDamage`
  (params (Damage :type "Float (single-precision)"))
  (set `self.Health` (- (`self.Health`) Damage)))

(event `/Game/Chris/Interfaces/DamageableInterface.Damage`
  (params (`Damage Amount` :type "Float (single-precision)"))
  (set `self.Health` (- (`self.Health`) `Damage Amount`)))

(event `/Game/Chris/Interfaces/DamageableInterface.Electrocute`
  (params (DamageAmount :type "Float (single-precision)") (Duration :type "Float (single-precision)") (Instakill :type Boolean))
  (bind _mesh (`self.Mesh`))
  (`|ExecutionSequence`
    (:`then_0`
      (if (<= (`KismetArrayLibrary.Array_Length` (`self.ParticleSystems`)) 3)
        (bind _returnvalue (`GameplayStatics.SpawnEmitterAttached` "/Game/Chris/Particles/P_SparkOnBones.P_SparkOnBones" _mesh "None" (0.0 0.0 0.0) (struct) (0.1 0.1 0.1)))
        (`KismetArrayLibrary.Array_Add` (`self.ParticleSystems`) _returnvalue)
        (`ParticleSystemComponent.SetActorParameter` _returnvalue "BoneSocketActor" (`ActorComponent.GetOwner` _mesh))
        (`self.PauseAI` true)))
    (:`then_1`
      (set `self.Instakill` Instakill))
    (:`then_2`
      (set `self.DOT_Amount` (/ DamageAmount Duration))
      (set `self.DOT_Duration` Duration)
      (set `self.DOT_Elapsed` 0.0)
      (bind _returnvalue_2 (`KismetSystemLibrary.K2_SetTimerDelegate` (delegate `DOT`) 1.0 true))
      (set `self.DOT_Timer` _returnvalue_2)
      (set `self.StartDOTTimer` true))))

(event `/Game/Chris/Interfaces/DamageableInterface.DamageOverTime`
  (params (`Damage Amount` :type "Float (single-precision)") (Duration :type "Float (single-precision)"))
  (if (not (`self.StartDOTTimer`))
    (set `self.DOT_Amount` (/ `Damage Amount` Duration))
    (set `self.DOT_Duration` Duration)
    (bind _returnvalue (`KismetSystemLibrary.K2_SetTimerDelegate` (delegate `DOT`) 1.0 true))
    (set `self.DOT_Timer` _returnvalue)
    (set `self.StartDOTTimer` true)))

(event `DOT`
  (bind _particlesystems (`self.ParticleSystems`))
  (bind _iscompleted (`self.ApplyDOT` (`self.DOT_Timer`)))
  (if _iscompleted
    (for _array_element _particlesystems
      (if (`KismetSystemLibrary.IsValid` _array_element)
        (`ActorComponent.Deactivate` _array_element)
        (`KismetSystemLibrary.Delay` 0.2)
        (`KismetArrayLibrary.Array_RemoveItem` _particlesystems _array_element)))
    (`self.PauseAI` false)
    (if (`self.Instakill`)
      (set `self.Health` 0.0))))

(event `/Game/Chris/Interfaces/DamageableInterface.SetOnFire`
  (params (`Damage Amount` :type "Float (single-precision)") (Duration :type "Float (single-precision)"))
  (bind _mesh (`self.Mesh`))
  (`|ExecutionSequence`
    (:`then_0`
      (if (<= (`KismetArrayLibrary.Array_Length` (`self.ParticleSystems`)) 3)
        (bind _returnvalue (`GameplayStatics.SpawnEmitterAttached` "/Game/Chris/Particles/P_FireOnBones.P_FireOnBones" _mesh "None" (0.0 0.0 0.0) (struct) (0.1 0.1 0.1)))
        (`KismetArrayLibrary.Array_Add` (`self.ParticleSystems`) _returnvalue)
        (`ParticleSystemComponent.SetActorParameter` _returnvalue "BoneSocketActor" (`ActorComponent.GetOwner` _mesh))))
    (:`then_1`
      (if (not (`self.StartDOTTimer`))
        (set `self.DOT_Amount` (/ `Damage Amount` Duration))
        (set `self.DOT_Duration` Duration)
        (bind _returnvalue_2 (`KismetSystemLibrary.K2_SetTimerDelegate` (delegate `DOT`) 1.0 true))
        (set `self.DOT_Timer` _returnvalue_2)
        (set `self.StartDOTTimer` true)))))

(event `self.ReceiveTick`
  (params (DeltaSeconds :type "Float (single-precision)"))
  (`|ExecutionSequence`
    (:`then_0`
      (`self.CheckForDeath`)
      (if (`self.IsDead`)
        (`self.StartRagdoll` (`self.NeedsRemoval`))
        (`/Engine/EditorBlueprintResources/StandardMacros.DoOnce` false
          (:`Completed`
            (for _array_element (`self.ParticleSystems`)
              (if (`KismetSystemLibrary.IsValid` _array_element)
                (`ActorComponent.Deactivate` _array_element)))))))
    (:`then_1`
      (`self.ActorDecay` DeltaSeconds))
    (:`then_2`
      (`self.IncrementDOTTimer` DeltaSeconds))))

(event `/Game/Chris/Interfaces/DamageableInterface.Freeze`
  (params (Duration :type "Float (single-precision)"))
  (`|ExecutionSequence`
    (:`then_0`
      (`/Engine/EditorBlueprintResources/StandardMacros.DoOnce` false
        (:`Completed`
          (bind _output_get (set `self.TemporaryMaterialHold` (`MeshComponent.GetMaterials` (`self.Mesh`))))
          (for (_ _array_index) _output_get
            (`PrimitiveComponent.SetMaterial` (`self.Mesh`) _array_index "/Game/Chris/Materials/Instances/Props/MI_Ice.MI_Ice"))
          (`self.PauseAI` true))))
    (:`then_1`
      (bind _output_get_2 (set `self.Freeze_Duration` Duration))
      (bind _returnvalue (`KismetSystemLibrary.K2_SetTimerDelegate` (delegate `Unfreeze`) _output_get_2))
      (set `self.Freeze_Timer` _returnvalue))))

(event `Unfreeze`
  (for (_array_element _array_index) (`self.TemporaryMaterialHold`)
    (`PrimitiveComponent.SetMaterial` (`self.Mesh`) _array_index _array_element))
  (`self.PauseAI` false))

(fn `ActorDecay`
  (params (`Delta Time` :type "Float (double-precision)"))
  (if (`self.NeedsRemoval`)
    (bind _output_get (set `self.CurrentDecayTime` (- (`self.CurrentDecayTime`) `Delta Time`)))
    (bind _onscreen (`self.IsActorOnScreen`))
    (if _onscreen
      (set `self.CurrentDecayTime` (`self.DecayTime`))
      (elif (<= _output_get 0.0)
        (`self.K2_DestroyActor`)))))

(fn `ApplyDOT`
  (params (`Timer Handle` :type "TimerHandle Structure"))
  (returns (IsCompleted :type Boolean))
  (locals (NewLocalVar_0 :type "Float (double-precision)" :default 0.0))
  (set `self.Health` (- (`self.Health`) (`self.DOT_Amount`)))
  (if (>= (`self.DOT_Elapsed`) (`self.DOT_Duration`))
    (`KismetSystemLibrary.K2_ClearAndInvalidateTimerHandle` `Timer Handle`)
    (set `self.StartDOTTimer` false)
    (set `self.DOT_Elapsed` 0.0)
    (return true)
    (else
      (return false))))

(fn `CheckForDeath`
  (returns (IsDead :type Boolean))
  (locals (`Temp Controller Ref` :type "AIController Object Reference"))
  (if (`self.Unpossessed`)
    _
    (elif (and (<= (`self.Health`) 0.0) (not (`self.NeedsRemoval`)))
      (if (not (`self.Unpossessed`))
        (`self.K2_DestroyActor` (`AIBlueprintHelperLibrary.GetAIController` self))
        (set `self.Unpossessed` true)
        (`PrimitiveComponent.SetCollisionEnabled` (`self.CapsuleComponent`) "NoCollision")
        (bind _output_get (set `self.IsDead` true))
        (return _output_get)))))

(fn `IncrementDOTTimer`
  (params (DeltaTime :type "Float (double-precision)"))
  (if (`self.StartDOTTimer`)
    (set `self.DOT_Elapsed` (+ DeltaTime (`self.DOT_Elapsed`)))))

(fn `IsActorOnScreen`
  (returns (OnScreen :type Boolean))
  (bind (_x _y) (`KismetMathLibrary.BreakVector2D` (`WidgetLayoutLibrary.GetViewportSize`)))
  (bind (_x_2 _y_2) (`KismetMathLibrary.BreakVector2D` (`PlayerController.ProjectWorldLocationToScreen` (`GameplayStatics.GetPlayerController` 0) (`SceneComponent.K2_GetComponentLocation` (`self.Mesh`)) false)))
  (return (and (> _x_2 0.0) (> _y_2 0.0) (< _x_2 _x) (< _y_2 _y))))

(fn `PauseAI`
  (params (ShouldPause :type Boolean))
  (bind _charactermovement (`self.CharacterMovement`))
  (bind _returnvalue (`AIBlueprintHelperLibrary.GetBlackboard` self))
  (if ShouldPause
    (`BlackboardComponent.SetValueAsBool` (`AIBlueprintHelperLibrary.GetBlackboard` self) (`self.FreezeKey`) true)
    (set `self.TemporaryMaxSpeedHold` (`CharacterMovementComponent.MaxWalkSpeed` _charactermovement))
    (set `CharacterMovementComponent.MaxWalkSpeed` 0.0 _charactermovement)
    (set `SkeletalMeshComponent.bPauseAnims` true (`self.Mesh`))
    (else
      (set `SkeletalMeshComponent.bPauseAnims` false (`self.Mesh`))
      (set `CharacterMovementComponent.MaxWalkSpeed` (`self.TemporaryMaxSpeedHold`) (`self.CharacterMovement`))
      (if (`KismetSystemLibrary.IsValid` _returnvalue)
        (`BlackboardComponent.SetValueAsBool` _returnvalue (`self.FreezeKey`) false)))))

(fn `SetEnemySearchLocation`
  (params (SearchLocation :type "Vector Structure"))
  (locals (EnemyLocationKey :type Name :default "EnemyLocation"))
  (`BlackboardComponent.SetValueAsVector` (`AIBlueprintHelperLibrary.GetBlackboard` self) (`local.EnemyLocationKey`) SearchLocation))

(fn `StartRagdoll`
  (params (Condition :type Boolean))
  (bind _mesh (`self.Mesh`))
  (if Condition
    (`/Engine/EditorBlueprintResources/StandardMacros.DoOnce` false
      (:`Completed`
        (`PrimitiveComponent.SetCollisionProfileName` _mesh "Ragdoll")
        (`PrimitiveComponent.SetSimulatePhysics` _mesh true)
        (return)))))

(fn `UserConstructionScript`)