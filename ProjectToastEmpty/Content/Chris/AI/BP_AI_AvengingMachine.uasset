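; AI-controlled Avenging Machine enemy that fires soda can projectiles at its blackboard target.
; Shoot spawns an enlarged BP_SodaCanProjectile just above the left or right hand socket, chosen by a flag.
; It then pushes the can's capsule with a force aimed straight at the target's current location.
; The Shoot call comes from outside this file, as the event graph holds no active logic.
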(fn `Shoot`
  (params (IsLeft :type Boolean))
  (locals (Target :type Name :default "Enemy") (SodaCan :type "/Game/Chris/Props/Weapons/BP_SodaCanProjectile Object Reference") (SpawnTransform :type "Transform Structure"))
  (bind _returnvalue (`KismetMathLibrary.MakeVector` 2.0 2.0 2.0))
  (bind _mesh (`self.Mesh`))
  (bind _rotation (.rotation (`SceneComponent.GetSocketTransform` _mesh (`self.LeftHandSocket`) "RTS_World")))
  (bind _rotation_2 (.rotation (`SceneComponent.GetSocketTransform` _mesh (`self.RightHandSocket`) "RTS_World")))
  (if IsLeft
    (set `local.SpawnTransform` (`KismetMathLibrary.MakeTransform` (+ (.location (`SceneComponent.GetSocketTransform` _mesh (`self.LeftHandSocket`) "RTS_World")) (* (`KismetMathLibrary.GetUpVector` _rotation) 5.0)) _rotation _returnvalue))
    (else
      (set `local.SpawnTransform` (`KismetMathLibrary.MakeTransform` (+ (.location (`SceneComponent.GetSocketTransform` _mesh (`self.RightHandSocket`) "RTS_World")) (* (`KismetMathLibrary.GetUpVector` _rotation_2) 5.0)) _rotation_2 _returnvalue))))
  (bind _returnvalue_2 (`|SpawnActorFromClass` "/Game/Chris/Props/Weapons/BP_SodaCanProjectile.BP_SodaCanProjectile_C" (`local.SpawnTransform`) "Undefined" "OverrideRootScale" null null))
  (bind _output_get (set `local.SodaCan` _returnvalue_2))
  (bind _asactor (cast `Actor` (`BlackboardComponent.GetValueAsObject` (`AIBlueprintHelperLibrary.GetBlackboard` (`self.GetController`)) (`local.Target`))))
  (`PrimitiveComponent.AddForce` (`/Game/Chris/Props/Weapons/BP_SodaCanProjectile.Capsule` _output_get) (* (`KismetMathLibrary.GetDirectionUnitVector` (`SceneComponent.K2_GetComponentLocation` (`/Game/Chris/Props/Weapons/BP_SodaCanProjectile.Capsule` _output_get)) (`self.K2_GetActorLocation` _asactor)) (`self.ShootingForce`)) "None" false))

(fn `UserConstructionScript`
  (`parent.UserConstructionScript`))