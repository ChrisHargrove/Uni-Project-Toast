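; Hovering AI bot that signals an alarm state and calls in AI reinforcements when alarmed.
; Construction attaches the eye light and hover effect to mesh sockets and creates a dynamic glow material, while BeginPlay starts an attached hover sound.
; ToggleAlarmed acts only on state changes, recoloring light, material and effect.
; On alarm, it tries spawn points sorted by distance, passing the blackboard enemy's location, until one spawns.
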(event `self.ReceiveBeginPlay`
  (`GameplayStatics.SpawnSoundAttached` "/Game/Chris/Sounds/HoverBot_HoverSound.HoverBot_HoverSound" (`self.Mesh`) "None" (0.0 0.0 0.0) (struct) "SnapToTarget" true 1.0 1.0 0.0 "/Game/Chris/Sounds/AttenuationSettings/SoundAttentuation.SoundAttentuation" null))

(event `self.ReceiveTick`
  (params (DeltaSeconds :type "Float (single-precision)"))
  (`parent.ReceiveTick` DeltaSeconds))

(fn `ToggleAlarmed`
  (params (IsAlarmed :type Boolean))
  (locals (AlarmedLightColor :type "LinearColor Structure" :default (struct :`R` 1.0 :`A` 1.0)) (PassiveLightColor :type "LinearColor Structure" :default (struct :`R` 1.0 :`G` 1.0 :`B` 1.0 :`A` 1.0)) (SortedSpawnPoints :type "Array of Actor Object Reference") (EnemyKey :type Name :default "Enemy"))
  (bind _eyelight (`self.EyeLight`))
  (bind _alarmedlightcolor (`local.AlarmedLightColor`))
  (bind _mesh (`self.Mesh`))
  (bind _passivelightcolor (`local.PassiveLightColor`))
  (if (!= IsAlarmed (`self.IsAlarmed`))
    (if IsAlarmed
      (`LightComponent.SetLightColor` _eyelight _alarmedlightcolor true)
      (bind _asmaterial_instance_dynamic (cast `MaterialInstanceDynamic` (`PrimitiveComponent.GetMaterial` _mesh 0)))
      (`MaterialInstanceDynamic.SetVectorParameterValue` _asmaterial_instance_dynamic "GlowColor" _alarmedlightcolor)
      (`ParticleSystemComponent.SetColorParameter` (`self.HoverEffect`) "HoverColor" _alarmedlightcolor)
      (else
        (`LightComponent.SetLightColor` _eyelight _passivelightcolor true)
        (bind _asmaterial_instance_dynamic_2 (cast `MaterialInstanceDynamic` (`PrimitiveComponent.GetMaterial` _mesh 0)))
        (`MaterialInstanceDynamic.SetVectorParameterValue` _asmaterial_instance_dynamic_2 "GlowColor" _passivelightcolor)
        (`ParticleSystemComponent.SetColorParameter` (`self.HoverEffect`) "HoverColor" _passivelightcolor)))
    (bind _output_get (set `self.IsAlarmed` IsAlarmed))
    (if _output_get
      (bind _outarray (`CustomBlueprintFunctions.SortByDistance` self false (`self.SpawnPoints`)))
      (bind _output_get_2 (set `local.SortedSpawnPoints` _outarray))
      (for _array_element _output_get_2
        (bind _asactor (cast `Actor` (`BlackboardComponent.GetValueAsObject` (`AIBlueprintHelperLibrary.GetBlackboard` self) (`local.EnemyKey`))))
        (bind _asbp_ai_spawn_point (cast `/Game/Chris/AI/BP_AI_SpawnPoint` _array_element))
        (bind _hasspawned (`/Game/Chris/AI/BP_AI_SpawnPoint.SpawnAI` _asbp_ai_spawn_point (`self.K2_GetActorLocation` _asactor)))
        (if _hasspawned
          (break))))))

(fn `UserConstructionScript`
  (bind _mesh (`self.Mesh`))
  (`ParticleSystemComponent.SetColorParameter` (`self.HoverEffect`) "HoverColor" (struct :`R` 0.442708 :`G` 0.442708 :`B` 0.442708 :`A` 1.0))
  (`PrimitiveComponent.CreateDynamicMaterialInstance` (`self.Mesh`) 0 "/Game/Chris/Materials/Instances/Characters/MI_HooverBot.MI_HooverBot" "None")
  (`SceneComponent.K2_AttachToComponent` (`self.EyeLight`) _mesh "LightSocket" "KeepRelative" "KeepRelative" "KeepRelative" true)
  (`SceneComponent.K2_AttachToComponent` (`self.HoverEffect`) _mesh "SmokeEffectSocket" "KeepRelative" "KeepRelative" "KeepRelative" true)
  (`parent.UserConstructionScript`))