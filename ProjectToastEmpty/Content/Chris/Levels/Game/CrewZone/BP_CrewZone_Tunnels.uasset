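; BP_CrewZone_Tunnels is a tunnel section of the crew zone that links its child-actor valve wheels to fuel pipes.
; On BeginPlay it casts and stores four valve wheels, then passes each to its own group of straight and bent pipes through SetValveWheel.
; The Fire and Cryo names are crossed: Cryo wheel components fill the FireValve variables, and Fire components fill the CryoValve ones.
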(event `self.ReceiveBeginPlay`
  (`|ExecutionSequence`
    (:`then_0`
      (bind _asbp_valve_wheel (cast `/Game/Chris/Props/BP_ValveWheel` (`ChildActorComponent.ChildActor` (`self.BP_ValveWheel_Cryo_01`))))
      (bind _output_get (set `self.FireValve_01` _asbp_valve_wheel))
      (`|ExecutionSequence`
        (:`then_0`
          (bind _asbp_fuel_pipe (cast `/Game/Chris/Props/BP_FuelPipe` (`ChildActorComponent.ChildActor` (`self.BP_FuelPipe_01`))))
          (`/Game/Chris/Props/BP_FuelPipe.SetValveWheel` _asbp_fuel_pipe _output_get))
        (:`then_1`
          (bind _asbp_fuel_pipe_2 (cast `/Game/Chris/Props/BP_FuelPipe` (`ChildActorComponent.ChildActor` (`self.BP_FuelPipe_02`))))
          (`/Game/Chris/Props/BP_FuelPipe.SetValveWheel` _asbp_fuel_pipe_2 _output_get))
        (:`then_2`
          (bind _asbp_fuel_pipe_3 (cast `/Game/Chris/Props/BP_FuelPipe` (`ChildActorComponent.ChildActor` (`self.BP_FuelPipe_03`))))
          (`/Game/Chris/Props/BP_FuelPipe.SetValveWheel` _asbp_fuel_pipe_3 _output_get))
        (:`then_3`
          (bind _asbp_bent_fuel_pipe (cast `/Game/Chris/Props/BP_BentFuelPipe` (`ChildActorComponent.ChildActor` (`self.BP_BentFuelPipe_01`))))
          (`/Game/Chris/Props/BP_BentFuelPipe.SetValveWheel` _asbp_bent_fuel_pipe _output_get))
        (:`then_4`
          (bind _asbp_bent_fuel_pipe_2 (cast `/Game/Chris/Props/BP_BentFuelPipe` (`ChildActorComponent.ChildActor` (`self.BP_BentFuelPipe_02`))))
          (`/Game/Chris/Props/BP_BentFuelPipe.SetValveWheel` _asbp_bent_fuel_pipe_2 _output_get))
        (:`then_5`
          (bind _asbp_bent_fuel_pipe_3 (cast `/Game/Chris/Props/BP_BentFuelPipe` (`ChildActorComponent.ChildActor` (`self.BP_BentFuelPipe_03`))))
          (`/Game/Chris/Props/BP_BentFuelPipe.SetValveWheel` _asbp_bent_fuel_pipe_3 _output_get))))
    (:`then_1`
      (bind _asbp_valve_wheel_2 (cast `/Game/Chris/Props/BP_ValveWheel` (`ChildActorComponent.ChildActor` (`self.BP_ValveWheel_Fire_01`))))
      (bind _output_get_2 (set `self.CryoValve_01` _asbp_valve_wheel_2))
      (`|ExecutionSequence`
        (:`then_0`
          (bind _asbp_fuel_pipe_4 (cast `/Game/Chris/Props/BP_FuelPipe` (`ChildActorComponent.ChildActor` (`self.BP_FuelPipe_04`))))
          (`/Game/Chris/Props/BP_FuelPipe.SetValveWheel` _asbp_fuel_pipe_4 _output_get_2))
        (:`then_1`
          (bind _asbp_fuel_pipe_5 (cast `/Game/Chris/Props/BP_FuelPipe` (`ChildActorComponent.ChildActor` (`self.BP_FuelPipe_05`))))
          (`/Game/Chris/Props/BP_FuelPipe.SetValveWheel` _asbp_fuel_pipe_5 _output_get_2))
        (:`then_2`
          (bind _asbp_fuel_pipe_6 (cast `/Game/Chris/Props/BP_FuelPipe` (`ChildActorComponent.ChildActor` (`self.BP_FuelPipe_06`))))
          (`/Game/Chris/Props/BP_FuelPipe.SetValveWheel` _asbp_fuel_pipe_6 _output_get_2))
        (:`then_3`
          (bind _asbp_fuel_pipe_7 (cast `/Game/Chris/Props/BP_FuelPipe` (`ChildActorComponent.ChildActor` (`self.BP_FuelPipe_07`))))
          (`/Game/Chris/Props/BP_FuelPipe.SetValveWheel` _asbp_fuel_pipe_7 _output_get_2))
        (:`then_4`
          (bind _asbp_fuel_pipe_8 (cast `/Game/Chris/Props/BP_FuelPipe` (`ChildActorComponent.ChildActor` (`self.BP_FuelPipe_08`))))
          (`/Game/Chris/Props/BP_FuelPipe.SetValveWheel` _asbp_fuel_pipe_8 _output_get_2))
        (:`then_5`
          (bind _asbp_fuel_pipe_9 (cast `/Game/Chris/Props/BP_FuelPipe` (`ChildActorComponent.ChildActor` (`self.BP_FuelPipe_09`))))
          (`/Game/Chris/Props/BP_FuelPipe.SetValveWheel` _asbp_fuel_pipe_9 _output_get_2))
        (:`then_6`
          (bind _asbp_fuel_pipe_10 (cast `/Game/Chris/Props/BP_FuelPipe` (`ChildActorComponent.ChildActor` (`self.BP_FuelPipe_10`))))
          (`/Game/Chris/Props/BP_FuelPipe.SetValveWheel` _asbp_fuel_pipe_10 _output_get_2))
        (:`then_7`
          (bind _asbp_bent_fuel_pipe_4 (cast `/Game/Chris/Props/BP_BentFuelPipe` (`ChildActorComponent.ChildActor` (`self.BP_BentFuelPipe_04`))))
          (`/Game/Chris/Props/BP_BentFuelPipe.SetValveWheel` _asbp_bent_fuel_pipe_4 _output_get_2))
        (:`then_8`
          (bind _asbp_bent_fuel_pipe_5 (cast `/Game/Chris/Props/BP_BentFuelPipe` (`ChildActorComponent.ChildActor` (`self.BP_BentFuelPipe_05`))))
          (`/Game/Chris/Props/BP_BentFuelPipe.SetValveWheel` _asbp_bent_fuel_pipe_5 _output_get_2))
        (:`then_9`
          (bind _asbp_bent_fuel_pipe_6 (cast `/Game/Chris/Props/BP_BentFuelPipe` (`ChildActorComponent.ChildActor` (`self.BP_BentFuelPipe_06`))))
          (`/Game/Chris/Props/BP_BentFuelPipe.SetValveWheel` _asbp_bent_fuel_pipe_6 _output_get_2))))
    (:`then_2`
      (bind _asbp_valve_wheel_3 (cast `/Game/Chris/Props/BP_ValveWheel` (`ChildActorComponent.ChildActor` (`self.BP_ValveWheel_Fire_02`))))
      (bind _output_get_3 (set `self.CryoValve_02` _asbp_valve_wheel_3))
      (`|ExecutionSequence`
        (:`then_0`
          (bind _asbp_fuel_pipe_11 (cast `/Game/Chris/Props/BP_FuelPipe` (`ChildActorComponent.ChildActor` (`self.BP_FuelPipe_11`))))
          (`/Game/Chris/Props/BP_FuelPipe.SetValveWheel` _asbp_fuel_pipe_11 _output_get_3))
        (:`then_1`
          (bind _asbp_fuel_pipe_12 (cast `/Game/Chris/Props/BP_FuelPipe` (`ChildActorComponent.ChildActor` (`self.BP_FuelPipe_12`))))
          (`/Game/Chris/Props/BP_FuelPipe.SetValveWheel` _asbp_fuel_pipe_12 _output_get_3))
        (:`then_2`
          (bind _asbp_fuel_pipe_13 (cast `/Game/Chris/Props/BP_FuelPipe` (`ChildActorComponent.ChildActor` (`self.BP_FuelPipe_13`))))
          (`/Game/Chris/Props/BP_FuelPipe.SetValveWheel` _asbp_fuel_pipe_13 _output_get_3))
        (:`then_3`
          (bind _asbp_fuel_pipe_14 (cast `/Game/Chris/Props/BP_FuelPipe` (`ChildActorComponent.ChildActor` (`self.BP_FuelPipe_14`))))
          (`/Game/Chris/Props/BP_FuelPipe.SetValveWheel` _asbp_fuel_pipe_14 _output_get_3))
        (:`then_4`
          (bind _asbp_bent_fuel_pipe_7 (cast `/Game/Chris/Props/BP_BentFuelPipe` (`ChildActorComponent.ChildActor` (`self.BP_BentFuelPipe07`))))
          (`/Game/Chris/Props/BP_BentFuelPipe.SetValveWheel` _asbp_bent_fuel_pipe_7 _output_get_3))
        (:`then_5`
          (bind _asbp_bent_fuel_pipe_8 (cast `/Game/Chris/Props/BP_BentFuelPipe` (`ChildActorComponent.ChildActor` (`self.BP_BentFuelPipe_08`))))
          (`/Game/Chris/Props/BP_BentFuelPipe.SetValveWheel` _asbp_bent_fuel_pipe_8 _output_get_3))
        (:`then_6`
          (bind _asbp_bent_fuel_pipe_9 (cast `/Game/Chris/Props/BP_BentFuelPipe` (`ChildActorComponent.ChildActor` (`self.BP_BentFuelPipe_09`))))
          (`/Game/Chris/Props/BP_BentFuelPipe.SetValveWheel` _asbp_bent_fuel_pipe_9 _output_get_3))))
    (:`then_3`
      (bind _asbp_valve_wheel_4 (cast `/Game/Chris/Props/BP_ValveWheel` (`ChildActorComponent.ChildActor` (`self.BP_ValveWheel_Cryo_02`))))
      (bind _output_get_4 (set `self.FireValve_02` _asbp_valve_wheel_4))
      (`|ExecutionSequence`
        (:`then_0`
          (bind _asbp_fuel_pipe_15 (cast `/Game/Chris/Props/BP_FuelPipe` (`ChildActorComponent.ChildActor` (`self.BP_FuelPipe_15`))))
          (`/Game/Chris/Props/BP_FuelPipe.SetValveWheel` _asbp_fuel_pipe_15 _output_get_4))
        (:`then_1`
          (bind _asbp_fuel_pipe_16 (cast `/Game/Chris/Props/BP_FuelPipe` (`ChildActorComponent.ChildActor` (`self.BP_FuelPipe_16`))))
          (`/Game/Chris/Props/BP_FuelPipe.SetValveWheel` _asbp_fuel_pipe_16 _output_get_4))
        (:`then_2`
          (bind _asbp_fuel_pipe_17 (cast `/Game/Chris/Props/BP_FuelPipe` (`ChildActorComponent.ChildActor` (`self.BP_FuelPipe_17`))))
          (`/Game/Chris/Props/BP_FuelPipe.SetValveWheel` _asbp_fuel_pipe_17 _output_get_4))
        (:`then_3`
          (bind _asbp_fuel_pipe_18 (cast `/Game/Chris/Props/BP_FuelPipe` (`ChildActorComponent.ChildActor` (`self.BP_FuelPipe_18`))))
          (`/Game/Chris/Props/BP_FuelPipe.SetValveWheel` _asbp_fuel_pipe_18 _output_get_4))
        (:`then_4`
          (bind _asbp_fuel_pipe_19 (cast `/Game/Chris/Props/BP_FuelPipe` (`ChildActorComponent.ChildActor` (`self.BP_FuelPipe_19`))))
          (`/Game/Chris/Props/BP_FuelPipe.SetValveWheel` _asbp_fuel_pipe_19 _output_get_4))
        (:`then_5`
          (bind _asbp_fuel_pipe_20 (cast `/Game/Chris/Props/BP_FuelPipe` (`ChildActorComponent.ChildActor` (`self.BP_FuelPipe_20`))))
          (`/Game/Chris/Props/BP_FuelPipe.SetValveWheel` _asbp_fuel_pipe_20 _output_get_4))
        (:`then_6`
          (bind _asbp_fuel_pipe_21 (cast `/Game/Chris/Props/BP_FuelPipe` (`ChildActorComponent.ChildActor` (`self.BP_FuelPipe_21`))))
          (`/Game/Chris/Props/BP_FuelPipe.SetValveWheel` _asbp_fuel_pipe_21 _output_get_4))
        (:`then_7`
          (bind _asbp_bent_fuel_pipe_10 (cast `/Game/Chris/Props/BP_BentFuelPipe` (`ChildActorComponent.ChildActor` (`self.BP_BentFuelPipe_10`))))
          (`/Game/Chris/Props/BP_BentFuelPipe.SetValveWheel` _asbp_bent_fuel_pipe_10 _output_get_4))
        (:`then_8`
          (bind _asbp_bent_fuel_pipe_11 (cast `/Game/Chris/Props/BP_BentFuelPipe` (`ChildActorComponent.ChildActor` (`self.BP_BentFuelPipe_11`))))
          (`/Game/Chris/Props/BP_BentFuelPipe.SetValveWheel` _asbp_bent_fuel_pipe_11 _output_get_4))))))

(fn `UserConstructionScript`)