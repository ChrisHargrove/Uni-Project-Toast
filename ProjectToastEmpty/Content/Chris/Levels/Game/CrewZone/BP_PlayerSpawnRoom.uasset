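; BP_PlayerSpawnRoom is the player's spawn room, with a sliding door that unlocks once the player has a gun.
; On BeginPlay it caches the door and player, then links each of two child-actor valve wheels to its own set of straight and bent fuel pipes.
; Tick polls the player's HasGun flag through a Gate, which closes after unlocking the door so the check stops.
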(event `self.ReceiveBeginPlay`
  (bind _asbp_sliding_door (cast `/Game/Chris/Props/BP_SlidingDoor` (`ChildActorComponent.ChildActor` (`self.SlidingDoor_01`))))
  (set `self.SlidingDoor` _asbp_sliding_door)
  (bind _asbp_fpscharacter (cast `/Game/Chris/Characters/Character/BP_FPSCharacter` (`GameplayStatics.GetPlayerCharacter` 0)))
  (set `self.PlayerReference` _asbp_fpscharacter)
  (`|ExecutionSequence`
    (:`then_0`
      (bind _asbp_valve_wheel (cast `/Game/Chris/Props/BP_ValveWheel` (`ChildActorComponent.ChildActor` (`self.BP_ValveWheel_01`))))
      (`|ExecutionSequence`
        (:`then_0`
          (bind _asbp_fuel_pipe (cast `/Game/Chris/Props/BP_FuelPipe` (`ChildActorComponent.ChildActor` (`self.BP_FuelPipe_01`))))
          (`/Game/Chris/Props/BP_FuelPipe.SetValveWheel` _asbp_fuel_pipe _asbp_valve_wheel))
        (:`then_1`
          (bind _asbp_fuel_pipe_2 (cast `/Game/Chris/Props/BP_FuelPipe` (`ChildActorComponent.ChildActor` (`self.BP_FuelPipe_02`))))
          (`/Game/Chris/Props/BP_FuelPipe.SetValveWheel` _asbp_fuel_pipe_2 _asbp_valve_wheel))
        (:`then_2`
          (bind _asbp_fuel_pipe_3 (cast `/Game/Chris/Props/BP_FuelPipe` (`ChildActorComponent.ChildActor` (`self.BP_FuelPipe_03`))))
          (`/Game/Chris/Props/BP_FuelPipe.SetValveWheel` _asbp_fuel_pipe_3 _asbp_valve_wheel))
        (:`then_3`
          (bind _asbp_bent_fuel_pipe (cast `/Game/Chris/Props/BP_BentFuelPipe` (`ChildActorComponent.ChildActor` (`self.BP_BentFuelPipe_01`))))
          (`/Game/Chris/Props/BP_BentFuelPipe.SetValveWheel` _asbp_bent_fuel_pipe _asbp_valve_wheel))))
    (:`then_1`
      (bind _asbp_valve_wheel_2 (cast `/Game/Chris/Props/BP_ValveWheel` (`ChildActorComponent.ChildActor` (`self.BP_ValveWheel_02`))))
      (`|ExecutionSequence`
        (:`then_0`
          (bind _asbp_fuel_pipe_4 (cast `/Game/Chris/Props/BP_FuelPipe` (`ChildActorComponent.ChildActor` (`self.BP_FuelPipe_04`))))
          (`/Game/Chris/Props/BP_FuelPipe.SetValveWheel` _asbp_fuel_pipe_4 _asbp_valve_wheel_2))
        (:`then_1`
          (bind _asbp_fuel_pipe_5 (cast `/Game/Chris/Props/BP_FuelPipe` (`ChildActorComponent.ChildActor` (`self.BP_FuelPipe_05`))))
          (`/Game/Chris/Props/BP_FuelPipe.SetValveWheel` _asbp_fuel_pipe_5 _asbp_valve_wheel_2))
        (:`then_2`
          (bind _asbp_bent_fuel_pipe_2 (cast `/Game/Chris/Props/BP_BentFuelPipe` (`ChildActorComponent.ChildActor` (`self.BP_BentFuelPipe_02`))))
          (`/Game/Chris/Props/BP_BentFuelPipe.SetValveWheel` _asbp_bent_fuel_pipe_2 _asbp_valve_wheel_2))
        (:`then_3`
          (bind _asbp_bent_fuel_pipe_3 (cast `/Game/Chris/Props/BP_BentFuelPipe` (`ChildActorComponent.ChildActor` (`self.BP_BentFuelPipe_03`))))
          (`/Game/Chris/Props/BP_BentFuelPipe.SetValveWheel` _asbp_bent_fuel_pipe_3 _asbp_valve_wheel_2))))))

(event `self.ReceiveTick`
  (params (DeltaSeconds :type "Float (single-precision)"))
  (`|ExecutionSequence`
    (:`then_0`
      (`/Engine/EditorBlueprintResources/StandardMacros.Gate` false :!label _label
        (:`Exit`
          (if (`/Game/Chris/Characters/Character/BP_FPSCharacter.HasGun` (`self.PlayerReference`))
            (set `/Game/Chris/Props/BP_SlidingDoor.IsLocked` false (`self.SlidingDoor`))
            (goto _label :!via `Close`)))))))

(fn `UserConstructionScript`)